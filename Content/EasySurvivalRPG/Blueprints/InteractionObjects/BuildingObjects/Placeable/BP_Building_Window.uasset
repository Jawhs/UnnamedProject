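; A placeable window for the survival building system that mounts into the socket of a window frame building.
; Snap and build checks filter targets by building type and reject frames that already hold a window, and placement takes the socket transform.
; Attaching snaps the window to that socket and sets references on both actors.
; Saving stores the frame's SaveID under "WindowFrame"; loading resolves it and reattaches the window.
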(event `self.CheckAndAttachToTarget`
  (params (TargetObject :type "/Game/EasySurvivalRPG/Blueprints/InteractionObjects/BuildingObjects/Base/BP_Building_BuildingObject Object Reference"))
  ;[1 1 1] Overridden events.
  (bind _asbp_building_window_frame (cast `/Game/EasySurvivalRPG/Blueprints/InteractionObjects/BuildingObjects/Modular/BP_Building_WindowFrame` TargetObject))
  (set `/Game/EasySurvivalRPG/Blueprints/InteractionObjects/BuildingObjects/Modular/BP_Building_WindowFrame.WindowReference` self _asbp_building_window_frame)
  (set `self.WindowFrameReference` _asbp_building_window_frame)
  (bind _windowsocket (`/Game/EasySurvivalRPG/Blueprints/InteractionObjects/BuildingObjects/Modular/BP_Building_WindowFrame.WindowSocket` _asbp_building_window_frame))
  (`self.K2_SetActorTransform` (`SceneComponent.K2_GetComponentToWorld` _windowsocket) false true)
  (`self.K2_AttachToComponent` _windowsocket "None" "SnapToTarget" "SnapToTarget" "SnapToTarget"))

(fn `CheckBuildStatus`
  (params (TargetObject :type "/Game/EasySurvivalRPG/Blueprints/InteractionObjects/BuildingObjects/Base/BP_Building_BuildingObject Object Reference"))
  (returns (CanBuild :type Boolean))
  (return (not (`KismetSystemLibrary.IsValid` (`/Game/EasySurvivalRPG/Blueprints/InteractionObjects/BuildingObjects/Modular/BP_Building_WindowFrame.WindowReference` (cast `/Game/EasySurvivalRPG/Blueprints/InteractionObjects/BuildingObjects/Modular/BP_Building_WindowFrame` TargetObject :!pure true))))))

(fn `CheckSnap`
  (params (TargetObject :type "/Game/EasySurvivalRPG/Blueprints/InteractionObjects/BuildingObjects/Base/BP_Building_BuildingObject Object Reference"))
  (returns (Snap :type Boolean))
  (return (`|EnumEquality` (`/Game/EasySurvivalRPG/Blueprints/InteractionObjects/BuildingObjects/Base/BP_Building_BuildingObject.BuildingType` TargetObject) "NewEnumerator5")))

(fn `GetSnapPosition`
  (params (TargetObject :type "/Game/EasySurvivalRPG/Blueprints/InteractionObjects/BuildingObjects/Base/BP_Building_BuildingObject Object Reference") (InputRotation :type "Float (double-precision)") (HitLocation :type "Vector Structure") (GridMode :type Boolean) (SnappingMode :type Boolean))
  (returns (NewLocation :type "Vector Structure") (NewRotation :type "Rotator Structure"))
  (bind (_returnvalue_location _returnvalue_rotation) (`KismetMathLibrary.BreakTransform` (`SceneComponent.K2_GetComponentToWorld` (`/Game/EasySurvivalRPG/Blueprints/InteractionObjects/BuildingObjects/Modular/BP_Building_WindowFrame.WindowSocket` (cast `/Game/EasySurvivalRPG/Blueprints/InteractionObjects/BuildingObjects/Modular/BP_Building_WindowFrame` TargetObject :!pure true)))))
  (return _returnvalue_location _returnvalue_rotation))

(fn `LoadData_BPI`
  (params (SaveData :type "SaveGame Object Reference"))
  (returns (Success :type Boolean))
  (bind _success (`parent.LoadData_BPI` SaveData))
  (if _success
    (bind (_success_2 _actor) (message `/Game/EasySurvivalRPG/Blueprints/Interfaces/BPI_GameSave.GetSavedActorReferenceByID_BPI` SaveData (`self.SaveID`) "WindowFrame"))
    (bind _asbp_building_building_object (cast `/Game/EasySurvivalRPG/Blueprints/InteractionObjects/BuildingObjects/Base/BP_Building_BuildingObject` _actor)
      (:`then`
        (`self.CheckAndAttachToTarget` _asbp_building_building_object)
        (return true))
      (:`CastFailed`
        _)))
  (return false))

(fn `SaveData_BPI`
  (params (SaveData :type "SaveGame Object Reference"))
  (returns (Success :type Boolean))
  (bind _windowframereference (`self.WindowFrameReference`))
  (bind _success (`parent.SaveData_BPI` SaveData))
  (if _success
    (`/Engine/EditorBlueprintResources/StandardMacros.IsValid` _windowframereference
      (:`Is Valid`
        (bind _success_2 (message `/Game/EasySurvivalRPG/Blueprints/Interfaces/BPI_GameSave.SetReferencesSaveData_BPI` SaveData (`self.SaveID`) (make `/Game/EasySurvivalRPG/Blueprints/Structures/SaveData/STR_SaveData_Referencess` (`|MakeMap` "WindowFrame" (`/Game/EasySurvivalRPG/Blueprints/InteractionObjects/BuildingObjects/Base/BP_Building_BuildingObject.SaveID` _windowframereference) :!type "Name"))))
        (return _success_2))
      (:`Is Not Valid`
        _)))
  (return false))

(fn `UserConstructionScript`
  (`parent.UserConstructionScript`))