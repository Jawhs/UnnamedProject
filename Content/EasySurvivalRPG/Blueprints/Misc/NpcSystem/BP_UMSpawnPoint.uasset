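; Spawn point that spawns AI characters configured for the UniversalMonster system, up to a maximum count.
; On the server, a randomly staggered looping timer runs a sphere overlap for players to activate or deactivate the point.
; Each spawn receives roaming, spline path and behavior settings, patrols from this point and has its death tracked.
; Spawns arrive all at once or on a respawn timer, optionally joining the first one's formation.
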(event `self.ReceiveBeginPlay`
  (bind _proximitytime (`self.ProximityTime`))
  ;[1 1 1] Spawn Point Proximity Activation
  (`parent.ReceiveBeginPlay`)
  (`/Engine/EditorBlueprintResources/ActorMacros.Switch Has Authority`
    (:`Authority`
      (bind _returnvalue (`KismetSystemLibrary.K2_SetTimerDelegate` (delegate `ProximityCheck`) (`KismetMathLibrary.RandomFloatInRange` (`KismetMathLibrary.FMax` _proximitytime 1.0) (+ _proximitytime 1.0)) true))
      (set `self.ProximityTimer` _returnvalue))))

(event `ProximityCheck`
  (bind _isactivated (`self.IsActivated`))
  ;[1 1 1] Spawn Point Proximity Activation
  (bind (_outactors _returnvalue) (`KismetSystemLibrary.SphereOverlapActors` (`self.K2_GetActorLocation`) (`self.ProximityRadius`) (`|MakeArray` "ObjectTypeQuery3" :!type "EObjectTypeQuery Enum") "/Game/EasySurvivalRPG/Blueprints/Characters/Base/BP_Character_Player.BP_Character_Player_C"))
  (if _returnvalue
    (if (not _isactivated)
      (`self.ActivateSpawnPoint`))
    (elif _isactivated
      (`self.DeactivateSpawnPoint`))))

(event `self.TrySpawn`
  (bind _leader (`self.Leader`))
  (bind _spawnedcharacters (`self.SpawnedCharacters`))
  (bind _universalmonster (`/Game/UniversalMonster/Blueprints/BPFL_UMFunctions.GetUniversalMonster` (`|GetArrayItem` _spawnedcharacters)))
  (bind _universalmonster_2 (`/Game/UniversalMonster/Blueprints/BPFL_UMFunctions.GetUniversalMonster` (`|GetArrayItem` _spawnedcharacters (`KismetArrayLibrary.Array_LastIndex` _spawnedcharacters))))
  ;[1 1 1] Try to spawn characters.
  (if (< (`KismetArrayLibrary.Array_Length` (`self.SpawnedCharacters`)) (`self.MaxCount`)) :!label _label
    (`self.Spawn`)
    (if (`self.bUseFormation`)
      (if (> (`KismetArrayLibrary.Array_Length` _spawnedcharacters) 1)
        (`/Engine/EditorBlueprintResources/StandardMacros.IsValid` _universalmonster_2
          (:`Is Valid`
            (`/Game/UniversalMonster/Blueprints/BP_UniversalMonster.AddToGroup` _universalmonster_2 _leader))
          (:`Is Not Valid`
            _))
        (else
          (`/Engine/EditorBlueprintResources/StandardMacros.IsValid` _universalmonster
            (:`Is Valid`
              (set `self.Leader` _universalmonster)
              (`/Game/UniversalMonster/Blueprints/BP_UniversalMonster.ChangeFormation` _leader (`self.Formation`)))
            (:`Is Not Valid`
              _)))))
    (`self.CheckRespawn`)
    (if (`self.SpawnGroup`)
      (goto _label))))

(event `self.Spawn`
  (bind (_location _rotation) (`self.GetSpawnLocationAndRotation`))
  ;[1 1 1] Spawn character.
  (bind _returnvalue (`AIBlueprintHelperLibrary.SpawnAIFromClass` (`self.CharacterClass`) (`self.CharacterBehavior`) _location _rotation true))
  (bind _universalmonster (`/Game/UniversalMonster/Blueprints/BPFL_UMFunctions.GetUniversalMonster` _returnvalue))
  (`/Engine/EditorBlueprintResources/StandardMacros.IsValid` _universalmonster
    (:`Is Valid`
      (`self.SetUM` _universalmonster)
      (bind _umaic (`/Game/UniversalMonster/Blueprints/BP_UniversalMonster.UMAIC` _universalmonster)
        (:`then`
          (`/Game/UniversalMonster/AI/AIC_UniversalMonster.StartUM` _umaic _universalmonster))
        (:`else`)))
    (:`Is Not Valid`
      _))
  (bind _asbp_character_base (cast `/Game/EasySurvivalRPG/Blueprints/Characters/Base/BP_Character_Base` _returnvalue))
  (`/Game/EasySurvivalRPG/Blueprints/Characters/Base/BP_Character_Base.SetPatrolPoint` _asbp_character_base self)
  (add `/Game/EasySurvivalRPG/Blueprints/Characters/Base/BP_Character_Base.OnDeath` _asbp_character_base (`|CreateDelegate` :!event `CharacterDied`))
  (`KismetArrayLibrary.Array_Add` (`self.SpawnedCharacters`) _asbp_character_base)
  (if (and (not (`self.SpawnGroup`)) (< (`KismetArrayLibrary.Array_Length` (`self.SpawnedCharacters`)) (`self.MaxCount`)))
    (bind _returnvalue_2 (`KismetSystemLibrary.K2_SetTimerDelegate` (`|CreateDelegate` :!event `TrySpawn`) (`self.RespawnTime`)))
    (set `self.RespawnTimerHandle` _returnvalue_2)))

(event `SetUM`
  (params (UniversalMonster :type "/Game/UniversalMonster/Blueprints/BP_UniversalMonster Object Reference"))
  (bind _splinepath (`self.SplinePath`))
  (bind _returnvalue (`AIBlueprintHelperLibrary.GetBlackboard` (`/Game/UniversalMonster/Blueprints/BP_UniversalMonster.Actor` UniversalMonster)))
  ;[1 1 1] Change UM Values
  (set `/Game/UniversalMonster/Blueprints/BP_UniversalMonster.bEnableDebugging` (`self.bEnableDebugging`) UniversalMonster)
  (set `/Game/UniversalMonster/Blueprints/BP_UniversalMonster.bEnableDebugging` (`self.bEnableDebugLog`) UniversalMonster)
  (set `/Game/UniversalMonster/Blueprints/BP_UniversalMonster.Formation` (`self.Formation`) UniversalMonster)
  (set `/Game/UniversalMonster/Blueprints/BP_UniversalMonster.RoamingRadius` (`self.RoamingRadius`) UniversalMonster)
  (set `/Game/UniversalMonster/Blueprints/BP_UniversalMonster.WaitTime` (`self.WaitTime`) UniversalMonster)
  (set `/Game/UniversalMonster/Blueprints/BP_UniversalMonster.WaitVariance` (`self.WaitVariance`) UniversalMonster)
  (set `/Game/UniversalMonster/Blueprints/BP_UniversalMonster.bTurn45` (`self.bTurn45`) UniversalMonster)
  (set `/Game/UniversalMonster/Blueprints/BP_UniversalMonster.TurnRatio` (`self.TurnRatio`) UniversalMonster)
  (set `/Game/UniversalMonster/Blueprints/BP_UniversalMonster.SplinePath` _splinepath UniversalMonster)
  (set `/Game/UniversalMonster/Blueprints/BP_UniversalMonster.CurrentSplineIndex` (`self.CurrentSplineIndex`) UniversalMonster)
  (set `/Game/UniversalMonster/Blueprints/BP_UniversalMonster.bSplineReversed` (`self.bSplineReversed`) UniversalMonster)
  (set `/Game/UniversalMonster/Blueprints/BP_UniversalMonster.CharacterBT` (`self.CharacterBehavior`) UniversalMonster)
  (`/Engine/EditorBlueprintResources/StandardMacros.IsValid` _returnvalue
    (:`Is Valid`
      (`BlackboardComponent.SetValueAsObject` _returnvalue "SplinePath" _splinepath))))

(fn `UserConstructionScript`
  (`parent.UserConstructionScript`)
  (`SphereComponent.SetSphereRadius` (`self.Proximity`) (`self.ProximityRadius`) false))