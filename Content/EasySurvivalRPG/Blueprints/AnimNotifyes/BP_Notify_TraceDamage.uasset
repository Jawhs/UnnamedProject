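; BP_Notify_TraceDamage is an animation notify, named Trace_Damage, that triggers melee damage tracing on the animated actor.
; With Universal Monster integration and UseUMTrace enabled on a UM player or enemy, it sets weapon and offhand hitboxes from their meshes.
; It then starts a timed trace for each underscore-separated name in HitBoxName, defaulting non-positive durations.
; Otherwise, it falls back to the owner's TraceDealDamage interface message.
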(fn `GetNotifyName`
  (returns (ReturnValue :type String))
  (return "Trace_Damage"))

(fn `Received_Notify`
  (params (MeshComp :type "SkeletalMeshComponent Object Reference") (Animation :type "AnimSequenceBase Object Reference"))
  (returns (ReturnValue :type Boolean))
  (locals (Actor :type "Actor Object Reference") (UniversalMonster :type "/Game/UniversalMonster/Blueprints/BP_UniversalMonster Object Reference") (AnimNotifys :type "Array of String"))
  (bind _traceduration (`self.TraceDuration`))
  (bind _actor (`local.Actor`))
  ;[1 1 1] Try to deal damage.
  ;;[1 0 0] Universal Monster Integration
  ;;;[1 0 0] Universal Monster Integration: Added these Local Variables
  (bind _output_get (set `local.Actor` (`ActorComponent.GetOwner` MeshComp)))
  (bind _output_get_2 (set `local.UniversalMonster` (`/Game/UniversalMonster/Blueprints/BPFL_UMFunctions.GetUniversalMonster` _output_get)))
  (`/Engine/EditorBlueprintResources/StandardMacros.IsValid` _output_get_2
    (:`Is Valid`
      (set `local.AnimNotifys` (`KismetStringLibrary.ParseIntoArray` (`self.HitBoxName`) "_"))
      (bind _asbp_umcharacter_player (cast `/Game/EasySurvivalRPG/Blueprints/Characters/Base/BP_UMCharacter_Player` _actor)
        (:`then`
          (if (`/Game/EasySurvivalRPG/Blueprints/Characters/Base/BP_UMCharacter_Base.bUseUMTrace` _asbp_umcharacter_player)
            (`/Game/UniversalMonster/Blueprints/BP_UniversalMonster.SetupHitBox` (`local.UniversalMonster`) (`/Game/EasySurvivalRPG/Blueprints/Characters/Base/BP_UMCharacter_Player.Weapon` _asbp_umcharacter_player) (`/Game/EasySurvivalRPG/Blueprints/Characters/Base/BP_UMCharacter_Base.GetWeaponMesh` _asbp_umcharacter_player (`/Game/EasySurvivalRPG/Blueprints/Characters/Base/BP_UMCharacter_Base.WeaponSocket` _asbp_umcharacter_player)))
            (`/Game/UniversalMonster/Blueprints/BP_UniversalMonster.SetupHitBox` (`local.UniversalMonster`) (`/Game/EasySurvivalRPG/Blueprints/Characters/Base/BP_UMCharacter_Player.Offhand` _asbp_umcharacter_player) (`/Game/EasySurvivalRPG/Blueprints/Characters/Base/BP_UMCharacter_Base.GetWeaponMesh` _asbp_umcharacter_player (`/Game/EasySurvivalRPG/Blueprints/Characters/Base/BP_UMCharacter_Base.OffhandSocket` _asbp_umcharacter_player)))
            (for _array_element (`local.AnimNotifys`) :!label _label
              (`/Game/UniversalMonster/Blueprints/BP_UniversalMonster.MontageNotifyBegin` (`local.UniversalMonster`) (`KismetStringLibrary.Conv_StringToName` _array_element) (select `bool` (> _traceduration 0.0) :`false` 0.25 :`true` _traceduration)))
            (else
              (message `/Game/EasySurvivalRPG/Blueprints/Interfaces/BPI_Character.TraceDealDamage_BPI` (`local.Actor`) :!label _label_2))))
        (:`CastFailed`
          (bind _asbp_umcharacter_enemy (cast `/Game/EasySurvivalRPG/Blueprints/Characters/Base/BP_UMCharacter_Enemy` _actor)
            (:`then`
              (if (`/Game/EasySurvivalRPG/Blueprints/Characters/Base/BP_UMCharacter_Base.bUseUMTrace` _asbp_umcharacter_enemy)
                (`/Game/UniversalMonster/Blueprints/BP_UniversalMonster.SetupHitBox` (`local.UniversalMonster`) (`/Game/EasySurvivalRPG/Blueprints/Characters/Base/BP_UMCharacter_Enemy.Weapon` _asbp_umcharacter_enemy) (`/Game/EasySurvivalRPG/Blueprints/Characters/Base/BP_UMCharacter_Base.GetWeaponMesh` _asbp_umcharacter_enemy (`/Game/EasySurvivalRPG/Blueprints/Characters/Base/BP_UMCharacter_Base.WeaponSocket` _asbp_umcharacter_enemy)))
                (`/Game/UniversalMonster/Blueprints/BP_UniversalMonster.SetupHitBox` (`local.UniversalMonster`) (`/Game/EasySurvivalRPG/Blueprints/Characters/Base/BP_UMCharacter_Enemy.Offhand` _asbp_umcharacter_enemy) (`StaticMeshComponent.StaticMesh` (`/Game/EasySurvivalRPG/Blueprints/Characters/Base/BP_UMCharacter_Enemy.OffhandMesh` _asbp_umcharacter_enemy)))
                (goto _label)
                (else
                  (goto _label_2))))
            (:`CastFailed`
              (goto _label_2))))))
    (:`Is Not Valid`
      (goto _label_2)))
  (return true))