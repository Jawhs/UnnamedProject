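; Player character for EasySurvivalRPG that plugs the Universal Monster (UM) system into survival combat, with UseUMTrace gating the parent melee trace.
; UM hits resolve on the server into tree and mine harvesting, building repair or damage, and actor damage with headshots.
; Damage uses UM attack data or falls back to attributes, with crits and a tiredness penalty.
; Also exposes bullet info and survival stats, plus debug keys for editing saved factions.
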(event `self.TraceDealDamage_BPI`
  (bind _followcamera (`self.FollowCamera`))
  (bind _returnvalue (`SceneComponent.GetForwardVector` _followcamera))
  (bind _targetarmlength (`SpringArmComponent.TargetArmLength` (`self.CameraBoom`)))
  (bind _returnvalue_2 (+ (`SceneComponent.K2_GetComponentLocation` _followcamera) (* _returnvalue _targetarmlength)))
  (if (`self.bUseUMTrace`)
    (if (`self.IsLocallyControlled`)
      (`self.TraceDealDamage (Server)` _returnvalue_2 (+ _returnvalue_2 (* _returnvalue (+ _targetarmlength 700.0)))))
    (else
      (`parent.TraceDealDamage_BPI`))))

(event `self.TraceDealDamage (Server)`
  (params (TraceStart :type "Vector Structure") (TraceEnd :type "Vector Structure"))
  (if (not (`self.bUseUMTrace`))
    (`parent.TraceDealDamage (Server)` TraceStart TraceEnd)))

(event `Key|X`
  (params (Key :type "Key Structure"))
  (:`Pressed`
    (`self.ServerAddFaction` (make `/Game/UniversalMonster/Blueprints/Structs/S_Faction` "Test" true (`|MakeArray`)))))

(event `ServerAddFaction`
  (params (Faction :type "/Game/UniversalMonster/Blueprints/Structs/S_Faction Structure"))
  (`/Game/UniversalMonster/Blueprints/BP_UMSaveGame.AddFaction` (`/Game/UniversalMonster/Blueprints/BP_UMGlobal.UMSaveGame` (`/Game/UniversalMonster/Blueprints/BP_UniversalMonster.UMGlobal` (`/Game/UniversalMonster/Blueprints/BP_UMComponent.UniversalMonster` (`self.BP_UMComponent`)))) Faction))

(event `ServerRemoveFaction`
  (params (FactionName :type Name))
  (`/Game/UniversalMonster/Blueprints/BP_UMSaveGame.RemoveFaction` (`/Game/UniversalMonster/Blueprints/BP_UMGlobal.UMSaveGame` (`/Game/UniversalMonster/Blueprints/BP_UniversalMonster.UMGlobal` (`/Game/UniversalMonster/Blueprints/BP_UMComponent.UniversalMonster` (`self.BP_UMComponent`)))) FactionName))

(event `ServerAddReputation`
  (params (`Faction Name` :type Name) (`Target Faction` :type Name) (Amount :type "Float (double-precision)"))
  (`/Game/UniversalMonster/Blueprints/BP_UMSaveGame.AddReputation` (`/Game/UniversalMonster/Blueprints/BP_UMGlobal.UMSaveGame` (`/Game/UniversalMonster/Blueprints/BP_UniversalMonster.UMGlobal` (`/Game/UniversalMonster/Blueprints/BP_UMComponent.UniversalMonster` (`self.BP_UMComponent`)))) `Faction Name` `Target Faction` Amount))

(event `ServerSetFaction`
  (params (Faction :type Name))
  (set `/Game/UniversalMonster/Blueprints/BP_UniversalMonster.Faction` (make `DataTableRowHandle` "/Game/UniversalMonster/Blueprints/DataTables/DT_UMFactions.DT_UMFactions" Faction) (`/Game/UniversalMonster/Blueprints/BP_UMComponent.UniversalMonster` (`self.BP_UMComponent`))))

(event `Key|C`
  (params (Key :type "Key Structure"))
  (:`Pressed`
    (`self.ServerRemoveFaction` "Test")))

(event `ServerPrint`
  (bind (_arrayindex _arrayelement) (`/Engine/EditorBlueprintResources/StandardMacros.ReverseForEachLoop` (`/Game/UniversalMonster/Blueprints/BP_UMSaveGame.Factions` (`/Game/UniversalMonster/Blueprints/BP_UMGlobal.UMSaveGame` (`/Game/UniversalMonster/Blueprints/BP_UniversalMonster.UMGlobal` (`/Game/UniversalMonster/Blueprints/BP_UMComponent.UniversalMonster` (`self.BP_UMComponent`))))))
    (:`LoopBody`
      (set `self.Reputations` " | ")
      (bind (_factionname _isplayerfaction_ _reputations) (break `/Game/UniversalMonster/Blueprints/Structs/S_Faction` _arrayelement))
      (for _array_element _reputations
        (set `self.Reputations` (`KismetStringLibrary.Concat_StrStr` (`self.Reputations`) (`KismetStringLibrary.Conv_DoubleToString` _array_element) " | ")))
      (`KismetSystemLibrary.PrintString` (`KismetStringLibrary.Concat_StrStr` (`KismetStringLibrary.Conv_NameToString` _factionname) ": " (`self.Reputations`)) true true (struct :`G` 0.66 :`B` 1.0 :`A` 1.0) 20.0))))

(event `Key|V`
  (params (Key :type "Key Structure"))
  (:`Pressed`
    (`self.ServerPrint`)))

(event `Key|B`
  (params (Key :type "Key Structure"))
  (:`Pressed`
    (`self.ServerAddReputation` "Hostile" "Test" 1.0)))

(event `Key|N`
  (params (Key :type "Key Structure"))
  (:`Pressed`
    (`self.ServerAddReputation` "Hostile" "Test" -1.0)))

(fn `GetBaseDamage`
  (returns (Damage :type "Float (double-precision)") (DamageType :type "DamageType Class Reference"))
  (locals (LocalIsCriticalDamage :type Boolean) (bHasUMAttacks :type Boolean :default false))
  (bind _attributescomponent (`self.AttributesComponent`))
  (bind _bhasumattacks (`local.bHasUMAttacks`))
  (bind _value (`/Game/EasySurvivalRPG/Blueprints/Components/BP_AttributesComponent.GetAttributeValue` _attributescomponent (struct :`TagName` "EasyRPG.Attributes.Base.Damage")))
  (bind _universalmonster (`/Game/UniversalMonster/Blueprints/BP_UMComponent.UniversalMonster` (`self.BP_UMComponent`)))
  (bind ((`DataTableRow_135_476861394EC56407164A2DB09445D2FB` _datatablerow) (`DamageType_74_874766694C942001E647129C3E43F869` _damagetype) (`MinDamage_29_F81766C343A65D750068C9BE3944D6E3` _mindamage) (`MaxDamage_30_F6C1C2F747F381BA64BCABB31229A7DB` _maxdamage) (`CritChance_49_D8D544FA492ECA9A154C558913491C70` _critchance) (`CritMultiplier_50_AA303BD84936FC24F5C7A9AB55416B81` _critmultiplier)) (break `/Game/UniversalMonster/Blueprints/Structs/S_Attack` (`/Game/UniversalMonster/Blueprints/BP_UniversalMonster.Attack` _universalmonster)))
  (bind _returnvalue (`KismetMathLibrary.RandomFloatInRange` (select `bool` _bhasumattacks :`false` (* _value 0.8) :`true` _mindamage) (select `bool` _bhasumattacks :`false` (* _value 1.2) :`true` _maxdamage)))
  (bind _returnvalue_2 (select `bool` (`self.IsTired`) :`false` _returnvalue :`true` (* _returnvalue 0.5)))
  ;[1 1 1] Get base damage and damage type.
  (set `local.bHasUMAttacks` (> (`KismetArrayLibrary.Array_Length` (`/Game/UniversalMonster/Blueprints/BP_UniversalMonster.Attacks` _universalmonster)) 0))
  (bind _output_get (set `local.LocalIsCriticalDamage` (select `bool` (`local.bHasUMAttacks`) :`false` (<= (`KismetMathLibrary.RandomFloat`) (`/Game/EasySurvivalRPG/Blueprints/Components/BP_AttributesComponent.GetAttributeValue` _attributescomponent (struct :`TagName` "EasyRPG.Attributes.Base.CriticalChance"))) :`true` (`KismetMathLibrary.RandomBoolWithWeight` _critchance))))
  (return (select `bool` (`local.LocalIsCriticalDamage`) :`false` _returnvalue_2 :`true` (* (select `bool` (`local.bHasUMAttacks`) :`false` (`/Game/EasySurvivalRPG/Blueprints/Components/BP_AttributesComponent.GetAttributeValue` _attributescomponent (struct :`TagName` "EasyRPG.Attributes.Base.CriticalDamage")) :`true` _critmultiplier) _returnvalue_2)) (select `bool` _output_get :`false` _damagetype :`true` "/Game/EasySurvivalRPG/Blueprints/Misc/Other/BP_CriticalDamage.BP_CriticalDamage_C")))

(fn `GetBulletInfo`
  (returns (BulletInfo :type "/Game/UniversalMonster/Blueprints/Structs/S_BulletInfo Structure"))
  (bind _charactermovement (`self.CharacterMovement`))
  (bind _staticmesh (`self.GetWeaponMesh` (`self.WeaponSocket`)))
  (bind _returnvalue (`SceneComponent.K2_GetComponentToWorld` (`self.Mesh`)))
  (bind (_value _returnvalue_2) (`BlueprintMapLibrary.Map_Find` (`self.BulletInfo`) _staticmesh))
  (bind _returnvalue_3 (`StaticMesh.FindSocket` _staticmesh "Start"))
  (if _returnvalue_2
    (bind _structout (setmembers `/Game/UniversalMonster/Blueprints/Structs/S_BulletInfo` :`StructRef` _value :`Location` (`KismetMathLibrary.TransformLocation` _returnvalue (`StaticMeshSocket.RelativeLocation` _returnvalue_3)) :`Direction` (`KismetMathLibrary.GetForwardVector` (`KismetMathLibrary.TransformRotation` _returnvalue (`StaticMeshSocket.RelativeRotation` _returnvalue_3))) :`Gravity` (`KismetMathLibrary.MakeVector` 0.0 0.0 (* (`MovementComponent.GetGravityZ` _charactermovement) (`CharacterMovementComponent.GravityScale` _charactermovement))) :`Wind` (0.0 0.0 0.0)))
    (return _structout)
    (else
      (return))))

(fn `GetStat`
  (params (Stat :type "/Game/UniversalMonster/Blueprints/Enums/E_StatName Enum" :default "NewEnumerator0"))
  (returns (Value :type "Float (double-precision)"))
  (bind _health (`self.Health`))
  (bind _maxhealth (`self.MaxHealth`))
  (bind _energy (`self.Energy`))
  (bind _maxenergy (`self.MaxEnergy`))
  (bind _thirst (`self.Thirst`))
  (bind _maxthirst (`self.MaxThirst`))
  (bind _hunger (`self.Hunger`))
  (bind _maxhunger (`self.MaxHunger`))
  (bind _oxygen (`self.Oxygen`))
  (bind _maxoxygen (`self.MaxOxygen`))
  (return (select `/Game/UniversalMonster/Blueprints/Enums/E_StatName` Stat :`NewEnumerator0` _health :`NewEnumerator8` _maxhealth :`NewEnumerator1` (/ _health _maxhealth) :`NewEnumerator2` _energy :`NewEnumerator9` _maxenergy :`NewEnumerator3` (/ _energy _maxenergy) :`NewEnumerator4` _hunger :`NewEnumerator10` _maxhunger :`NewEnumerator5` (/ _hunger _maxhunger) :`NewEnumerator6` _thirst :`NewEnumerator11` _maxthirst :`NewEnumerator7` (/ _thirst _maxthirst) :`NewEnumerator12` _oxygen :`NewEnumerator13` _maxoxygen :`NewEnumerator14` (/ _oxygen _maxoxygen))))

(fn `SetStat`
  (params (Stat :type "/Game/UniversalMonster/Blueprints/Enums/E_StatName Enum" :default "NewEnumerator0") (Value :type "Float (double-precision)"))
  (returns (`bResult?` :type Boolean))
  (switch `/Game/UniversalMonster/Blueprints/Enums/E_StatName` Stat
    (:`NewEnumerator0`
      _)
    (:`NewEnumerator8`
      _)
    (:`NewEnumerator1`
      (return false))
    (:`NewEnumerator2`
      _)
    (:`NewEnumerator9`
      _)
    (:`NewEnumerator3`
      (return false))
    (:`NewEnumerator4`
      (set `self.Hunger` Value)
      (return true))
    (:`NewEnumerator10`
      (set `self.MaxHunger` Value)
      (return true))
    (:`NewEnumerator5`
      (return false))
    (:`NewEnumerator6`
      (set `self.Thirst` Value)
      (return true))
    (:`NewEnumerator11`
      (set `self.MaxThirst` Value)
      (return true))
    (:`NewEnumerator7`
      (return false))
    (:`NewEnumerator12`
      (set `self.Oxygen` Value)
      (return true))
    (:`NewEnumerator13`
      (set `self.MaxOxygen` Value)
      (return true))
    (:`NewEnumerator14`
      (return false)))
  (bind _bresult_ (`parent.SetStat` Stat Value))
  (return _bresult_))

(fn `UMHit`
  (params (UniversalMonster :type "/Game/UniversalMonster/Blueprints/BP_UniversalMonster Object Reference") (Attack :type "/Game/UniversalMonster/Blueprints/Structs/S_Attack Structure") (HitBox :type "BoxComponent Object Reference") (Projectile :type "/Game/UniversalMonster/Blueprints/BP_UMProjectile Object Reference") (Timer :type "/Game/UniversalMonster/Blueprints/BP_UMTimer Object Reference") (Bullet :type "/Game/UniversalMonster/Blueprints/Structs/S_BulletInfo Structure") (Hit :type "HitResult Structure"))
  (returns (`bResult?` :type Boolean))
  (`/Engine/EditorBlueprintResources/ActorMacros.Switch Has Authority`
    (:`Authority`
      (`self.UMTrace` Hit)
      (return true))))

(fn `UMTrace`
  (params (UMHit :type "HitResult Structure"))
  (locals (LocalTraceStart :type "Vector Structure") (LocalHit :type "HitResult Structure") (LocalHitActors :type "Array of Actor Object Reference") (LocalHitLocation :type "Vector Structure") (LocalActor :type "Actor Object Reference") (LocalSurfaceType :type "EPhysicalSurface Enum") (LocalTree :type "/Game/EasySurvivalRPG/Blueprints/InteractionObjects/Trees/BP_Tree_Base Object Reference") (LocalMine :type "/Game/EasySurvivalRPG/Blueprints/InteractionObjects/Mine/BP_Mine_Base Object Reference") (LocalBone :type Name :default "None"))
  (bind (_damage _damagetype) (`self.GetBaseDamage`))
  (bind (_damage_2 _damagetype_2) (`self.GetBaseDamage`))
  (bind _hotbarcontainer (`self.HotbarContainer`))
  (bind (_asbp_umcharacter_base _bsuccess) (cast `/Game/EasySurvivalRPG/Blueprints/Characters/Base/BP_UMCharacter_Base` (`local.LocalActor`) :!pure true))
  (bind _universalmonster (`/Game/UniversalMonster/Blueprints/BP_UMComponent.UniversalMonster` (`self.BP_UMComponent`)))
  (bind (_istool _tooltype) (`/Game/EasySurvivalRPG/Blueprints/Game/Libraries/BP_ItemsLibrary.ItemIsTool` (`/Game/EasySurvivalRPG/Blueprints/Components/BP_ContainerComponent.GetItem` _hotbarcontainer (`/Game/EasySurvivalRPG/Blueprints/Components/BP_HotbarComponent.SelectedItemSlot` _hotbarcontainer))))
  (bind _returnvalue (== (`local.LocalBone`) (select `bool` _bsuccess :`false` "head" :`true` (`/Game/EasySurvivalRPG/Blueprints/Characters/Base/BP_UMCharacter_Base.HeadBone` _asbp_umcharacter_base))))
  ;[1 1 1] Try to deal melee damage on the server.
  (bind _output_get (set `local.LocalHit` UMHit))
  (bind (_bblockinghit _binitialoverlap _time _distance _location _impactpoint _normal _impactnormal _physmat _hitactor _hitcomponent _hitbonename _hititem _faceindex _tracestart) (`GameplayStatics.BreakHitResult` _output_get))
  (if _bblockinghit
    (set `local.LocalBone` _hitbonename)
    (set `local.LocalTraceStart` _tracestart)
    (message `/Game/EasySurvivalRPG/Blueprints/Interfaces/BPI_Player.PlayHitReaction_BPI` (`self.GetController`))
    (`self.CheckToolHitAnimation`)
    (set `local.LocalHitLocation` _location)
    (bind _output_get_2 (set `local.LocalActor` _hitactor))
    (`KismetArrayLibrary.Array_AddUnique` (`local.LocalHitActors`) _output_get_2)
    (`/Engine/EditorBlueprintResources/StandardMacros.IsValid` _physmat
      (:`Is Valid`
        (set `local.LocalSurfaceType` (`PhysicalMaterial.SurfaceType` _physmat)))
      (:`Is Not Valid`
        _))
    ;;[1 1 1] Try to damage tree.
    (bind _asbp_instanced_component_tree_base (cast `/Game/EasySurvivalRPG/Blueprints/Components/InstancedComponents/BP_InstancedComponent_Tree_Base` _hitcomponent)
      (:`then`
        (`/Game/EasySurvivalRPG/Blueprints/Components/InstancedComponents/BP_InstancedComponent_Tree_Base.SpawnTree` _asbp_instanced_component_tree_base _hititem))
      (:`CastFailed`
        (bind _asbp_tree_base (cast `/Game/EasySurvivalRPG/Blueprints/InteractionObjects/Trees/BP_Tree_Base` (`local.LocalActor`))
          (:`then`
            (set `local.LocalTree` _asbp_tree_base)
            (`GameplayStatics.ApplyPointDamage` (`local.LocalActor`) (`self.GetWoodcuttingDamage`) (`local.LocalTraceStart`) (`local.LocalHit`) (`self.GetController`) self)
            (`self.PlaySoundAtLocation (Multicast)` (`self.GetImpactSound` (`local.LocalSurfaceType`)) (`local.LocalHitLocation`))
            (`self.TryToChangeItemDurability` (`self.InteractionItemContainer`) (`self.InteractionItemSlot`)))
          (:`CastFailed`
            ;;[1 1 1] Try to damage mine.
            (bind _asbp_instanced_component_mine_base (cast `/Game/EasySurvivalRPG/Blueprints/Components/InstancedComponents/BP_InstancedComponent_Mine_Base` _hitcomponent)
              (:`then`
                (`/Game/EasySurvivalRPG/Blueprints/Components/InstancedComponents/BP_InstancedComponent_Mine_Base.SpawnMine` _asbp_instanced_component_mine_base _hititem))
              (:`CastFailed`
                (bind _asbp_mine_base (cast `/Game/EasySurvivalRPG/Blueprints/InteractionObjects/Mine/BP_Mine_Base` (`local.LocalActor`))
                  (:`then`
                    (set `local.LocalMine` _asbp_mine_base)
                    (`GameplayStatics.ApplyPointDamage` (`local.LocalActor`) (`self.GetMiningDamage`) (`local.LocalTraceStart`) (`local.LocalHit`) (`self.GetController`) self)
                    (`self.PlaySoundAtLocation (Multicast)` (`self.GetImpactSound` (`local.LocalSurfaceType`)) (`local.LocalHitLocation`))
                    (`self.TryToChangeItemDurability` (`self.InteractionItemContainer`) (`self.InteractionItemSlot`)))
                  (:`CastFailed`
                    ;;[1 1 1] Try to deal damage to building or repair it if mallet is equiped.
                    (bind _asbp_building_building_object (cast `/Game/EasySurvivalRPG/Blueprints/InteractionObjects/BuildingObjects/Base/BP_Building_BuildingObject` (`local.LocalActor`))
                      (:`then`
                        (bind _asplayer_controller (cast `PlayerController` (`self.GetController`))
                          (:`then`
                            (bind _result (`/Game/EasySurvivalRPG/Blueprints/InteractionObjects/BuildingObjects/Base/BP_Building_BuildingObject.CheckOwnership` _asbp_building_building_object _asplayer_controller))
                            (if _result
                              (if (and _istool (`|EnumEquality` _tooltype "NewEnumerator3"))
                                (`/Game/EasySurvivalRPG/Blueprints/InteractionObjects/BuildingObjects/Base/BP_Building_BuildingObject.Repair` _asbp_building_building_object _asplayer_controller)
                                (else
                                  (`GameplayStatics.ApplyPointDamage` (`local.LocalActor`) _damage_2 (`local.LocalTraceStart`) (`local.LocalHit`) (`self.GetController`) self _damagetype_2 :!label _label)))
                              (else
                                (goto _label))))
                          (:`CastFailed`
                            (goto _label)))
                        (`self.PlaySoundAtLocation (Multicast)` (`self.GetImpactSound` (`local.LocalSurfaceType`)) (`local.LocalHitLocation`))
                        (`self.TryToChangeItemDurability` (`self.InteractionItemContainer`) (`self.InteractionItemSlot`)))
                      (:`CastFailed`
                        ;;[1 1 1] Try to damage characters and other actors.
                        (bind _ascharacter (cast `Character` (`local.LocalActor`))
                          (:`then`
                            (if (`Actor.bCanBeDamaged` _ascharacter)
                              (bind _state (message `/Game/EasySurvivalRPG/Blueprints/Interfaces/BPI_Character.GetInteractionState_BPI` _ascharacter "NewEnumerator3"))
                              (if _state
                                (set `local.LocalSurfaceType` "SurfaceType3"))
                              (`GameplayStatics.ApplyPointDamage` (`local.LocalActor`) (select `bool` _returnvalue :`false` _damage :`true` (* _damage (select `bool` (`KismetArrayLibrary.Array_IsValidIndex` (`/Game/UniversalMonster/Blueprints/BP_UniversalMonster.Attacks` _universalmonster)) :`false` (`/Game/EasySurvivalRPG/Blueprints/Components/BP_AttributesComponent.GetAttributeValue` (`self.AttributesComponent`) (struct :`TagName` "EasyRPG.Attributes.Base.CriticalDamage")) :`true` (`.CritMultiplier_50_AA303BD84936FC24F5C7A9AB55416B81` (break `/Game/UniversalMonster/Blueprints/Structs/S_Attack` (`/Game/UniversalMonster/Blueprints/BP_UniversalMonster.Attack` _universalmonster)))))) (`local.LocalTraceStart`) (`local.LocalHit`) (`self.GetController`) self (select `bool` _returnvalue :`false` _damagetype :`true` "/Game/EasySurvivalRPG/Blueprints/Misc/Other/BP_CriticalDamage.BP_CriticalDamage_C") :!label _label_2)
                              (`self.PlaySoundAtLocation (Multicast)` (`self.GetImpactSound` (`local.LocalSurfaceType`)) (`local.LocalHitLocation`))
                              (`self.TryToChangeItemDurability` (`self.InteractionItemContainer`) (`self.InteractionItemSlot`))
                              ;[1 1 1] Headshot
                              (if _returnvalue
                                (message `/Game/EasySurvivalRPG/Blueprints/Interfaces/BPI_Player.HeadshotNotification_BPI` self))))
                          (:`CastFailed`
                            (goto _label_2)))))))))))))))

(fn `UserConstructionScript`
  (bind _offhandmesh (`self.OffhandMesh`))
  (bind _weapon (`self.Weapon`))
  (`parent.UserConstructionScript`)
  (`SceneComponent.K2_AttachToComponent` _weapon (`self.Mesh`) (`self.WeaponSocket`) "KeepRelative" "KeepRelative" "KeepRelative" true)
  (`SceneComponent.K2_SetRelativeTransform` _weapon (`self.WeaponTransform`) false false)
  (`SceneComponent.K2_AttachToComponent` _offhandmesh (`self.Mesh`) (`self.OffhandSocket`) "KeepRelative" "KeepRelative" "KeepRelative" true)
  (`SceneComponent.K2_SetRelativeTransform` _offhandmesh (`self.OffhandTransform`) false false)
  (`|ExecutionSequence`
    (:`then_0`
      (if (not (`self.bIsModular`))
        (`SceneComponent.SetVisibility` (`self.PantsMesh`) false false)
        (`SceneComponent.SetVisibility` (`self.HandsMesh`) false false)
        (`SceneComponent.SetVisibility` (`self.BodyMesh`) false false)
        (`SceneComponent.SetVisibility` (`self.HeadMesh`) false false)
        (`SceneComponent.SetVisibility` (`self.FeetMesh`) false false)))
    (:`then_1`
      (if (not (`self.bShowOffhand`))
        (`SceneComponent.SetVisibility` (`self.OffhandMesh`) false false)))))