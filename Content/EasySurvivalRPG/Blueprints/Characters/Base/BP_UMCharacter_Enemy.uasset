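; Enemy character base that plugs the Universal Monster (UM) component into EasySurvivalRPG combat, with socketed weapon and offhand meshes.
; UMHit runs UMTrace on the server to damage trees, mines, buildings (or repair them) and other actors, with head-bone crit hits.
; Damage rolls use UM attack data, falling back to RPG attributes.
; Death drops loot, ragdolls if no UM death entry exists, and disables AI; server tick regenerates health and energy.
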(event `self.TraceDealDamage (Server)`
  (params (TraceStart :type "Vector Structure") (TraceEnd :type "Vector Structure"))
  (if (not (`self.bUseUMTrace`))
    (`parent.TraceDealDamage (Server)` TraceStart TraceEnd)))

(fn `Death`
  (params (KillerController :type "Controller Object Reference"))
  (returns (Success :type Boolean))
  (bind _universalmonster (`/Game/UniversalMonster/Blueprints/BP_UMComponent.UniversalMonster` (`self.BP_UMComponent`)))
  ;[1 1 1] Actions when the undead dies.
  (`self.DropDeathLoot`)
  (`self.MakeDeathLoot`)
  (if (not (`.ReturnValue` (`BlueprintMapLibrary.Map_Find` (`/Game/UniversalMonster/Blueprints/BP_UniversalMonster.Death` _universalmonster) (`/Game/UniversalMonster/Blueprints/BP_UniversalMonster.CurrentState` _universalmonster))))
    (`self.EnableRagdoll (Multicast)`))
  (`self.DeleteMark (Multicast)`)
  ;[1 1 1] Actions when the character dies.
  (set `self.IsAlive` false)
  (set `self.bCanBeDamaged` false)
  (`self.OnDeath` self KillerController)
  (message `/Game/EasySurvivalRPG/Blueprints/Interfaces/BPI_Player.PlayerKillCharacter_BPI` KillerController self)
  (`self.StopAnimation (Multicast)` 0.0)
  (`KismetSystemLibrary.K2_SetTimerDelegate` (`|CreateDelegate` :!event `DestroyCharacterOnDeath`) (`self.DestroyCharacterTimer`))
  (`/Engine/EditorBlueprintResources/StandardMacros.IsValid` (`AIBlueprintHelperLibrary.GetAIController` self)
    (:`Is Valid`
      (`self.DisableAI`))
    (:`Is Not Valid`
      _))
  (return false))

(fn `GetBaseDamage`
  (returns (Damage :type "Float (double-precision)") (DamageType :type "DamageType Class Reference"))
  (locals (LocalIsCriticalDamage :type Boolean) (bHasUMAttacks :type Boolean :default false))
  (bind _attributescomponent (`self.AttributesComponent`))
  (bind _bhasumattacks (`local.bHasUMAttacks`))
  (bind _value (`/Game/EasySurvivalRPG/Blueprints/Components/BP_AttributesComponent.GetAttributeValue` _attributescomponent (struct :`TagName` "EasyRPG.Attributes.Base.Damage")))
  (bind _universalmonster (`/Game/UniversalMonster/Blueprints/BP_UMComponent.UniversalMonster` (`self.BP_UMComponent`)))
  (bind ((`DataTableRow_135_476861394EC56407164A2DB09445D2FB` _datatablerow) (`DamageType_74_874766694C942001E647129C3E43F869` _damagetype) (`MinDamage_29_F81766C343A65D750068C9BE3944D6E3` _mindamage) (`MaxDamage_30_F6C1C2F747F381BA64BCABB31229A7DB` _maxdamage) (`CritChance_49_D8D544FA492ECA9A154C558913491C70` _critchance) (`CritMultiplier_50_AA303BD84936FC24F5C7A9AB55416B81` _critmultiplier)) (break `/Game/UniversalMonster/Blueprints/Structs/S_Attack` (`/Game/UniversalMonster/Blueprints/BP_UniversalMonster.Attack` _universalmonster)))
  (bind _returnvalue (`KismetMathLibrary.RandomFloatInRange` (select `bool` _bhasumattacks :`false` (* _value 0.8) :`true` _mindamage) (select `bool` _bhasumattacks :`false` (* _value 1.2) :`true` _maxdamage)))
  ;[1 1 1] Get base damage and damage type.
  (set `local.bHasUMAttacks` (> (`KismetArrayLibrary.Array_Length` (`/Game/UniversalMonster/Blueprints/BP_UniversalMonster.Attacks` _universalmonster)) 0))
  (bind _output_get (set `local.LocalIsCriticalDamage` (select `bool` (`local.bHasUMAttacks`) :`false` (<= (`KismetMathLibrary.RandomFloat`) (`/Game/EasySurvivalRPG/Blueprints/Components/BP_AttributesComponent.GetAttributeValue` _attributescomponent (struct :`TagName` "EasyRPG.Attributes.Base.CriticalChance"))) :`true` (`KismetMathLibrary.RandomBoolWithWeight` _critchance))))
  (return (select `bool` (`local.LocalIsCriticalDamage`) :`false` _returnvalue :`true` (* (select `bool` _bhasumattacks :`false` (`/Game/EasySurvivalRPG/Blueprints/Components/BP_AttributesComponent.GetAttributeValue` _attributescomponent (struct :`TagName` "EasyRPG.Attributes.Base.CriticalDamage")) :`true` _critmultiplier) _returnvalue)) (select `bool` _output_get :`false` _damagetype :`true` "/Game/EasySurvivalRPG/Blueprints/Misc/Other/BP_CriticalDamage.BP_CriticalDamage_C")))

(fn `GetBulletInfo`
  (returns (BulletInfo :type "/Game/UniversalMonster/Blueprints/Structs/S_BulletInfo Structure"))
  (bind _weaponmesh (`self.WeaponMesh`))
  (bind _charactermovement (`self.CharacterMovement`))
  (bind _returnvalue (`SceneComponent.K2_GetComponentToWorld` _weaponmesh))
  (bind _staticmesh (`StaticMeshComponent.StaticMesh` _weaponmesh))
  (bind (_value _returnvalue_2) (`BlueprintMapLibrary.Map_Find` (`self.BulletInfo`) _staticmesh))
  (bind _returnvalue_3 (`StaticMesh.FindSocket` _staticmesh "Start"))
  (if _returnvalue_2
    (bind _structout (setmembers `/Game/UniversalMonster/Blueprints/Structs/S_BulletInfo` :`StructRef` _value :`Location` (`KismetMathLibrary.TransformLocation` _returnvalue (`StaticMeshSocket.RelativeLocation` _returnvalue_3)) :`Direction` (`KismetMathLibrary.GetForwardVector` (`KismetMathLibrary.TransformRotation` _returnvalue (`StaticMeshSocket.RelativeRotation` _returnvalue_3))) :`Gravity` (`KismetMathLibrary.MakeVector` 0.0 0.0 (* (`MovementComponent.GetGravityZ` _charactermovement) (`CharacterMovementComponent.GravityScale` _charactermovement))) :`Wind` (0.0 0.0 0.0)))
    (return _structout)
    (else
      (return))))

(fn `UMHit`
  (params (UniversalMonster :type "/Game/UniversalMonster/Blueprints/BP_UniversalMonster Object Reference") (Attack :type "/Game/UniversalMonster/Blueprints/Structs/S_Attack Structure") (HitBox :type "BoxComponent Object Reference") (Projectile :type "/Game/UniversalMonster/Blueprints/BP_UMProjectile Object Reference") (Timer :type "/Game/UniversalMonster/Blueprints/BP_UMTimer Object Reference") (Bullet :type "/Game/UniversalMonster/Blueprints/Structs/S_BulletInfo Structure") (Hit :type "HitResult Structure"))
  (returns (`bResult?` :type Boolean))
  (`/Engine/EditorBlueprintResources/ActorMacros.Switch Has Authority`
    (:`Authority`
      (`self.UMTrace` Hit)
      (return true))))

(fn `UMTrace`
  (params (UMHit :type "HitResult Structure"))
  (locals (LocalTraceStart :type "Vector Structure") (LocalHit :type "HitResult Structure") (LocalHitLocation :type "Vector Structure") (LocalActor :type "Actor Object Reference") (LocalSurfaceType :type "EPhysicalSurface Enum") (LocalTree :type "/Game/EasySurvivalRPG/Blueprints/InteractionObjects/Trees/BP_Tree_Base Object Reference") (LocalMine :type "/Game/EasySurvivalRPG/Blueprints/InteractionObjects/Mine/BP_Mine_Base Object Reference") (LocalBone :type Name))
  (bind (_damage _damagetype) (`self.GetBaseDamage`))
  (bind (_damage_2 _damagetype_2) (`self.GetBaseDamage`))
  (bind (_damage_3 _damagetype_3) (`self.GetBaseDamage`))
  (bind (_damage_4 _damagetype_4) (`self.GetBaseDamage`))
  (bind (_istool _tooltype) (`/Game/EasySurvivalRPG/Blueprints/Game/Libraries/BP_ItemsLibrary.ItemIsTool` (`self.WeaponItemData`)))
  (bind (_asbp_umcharacter_base _bsuccess) (cast `/Game/EasySurvivalRPG/Blueprints/Characters/Base/BP_UMCharacter_Base` (`local.LocalActor`) :!pure true))
  (bind _universalmonster (`/Game/UniversalMonster/Blueprints/BP_UMComponent.UniversalMonster` (`self.BP_UMComponent`)))
  (bind _returnvalue (== (`local.LocalBone`) (select `bool` _bsuccess :`false` "head" :`true` (`/Game/EasySurvivalRPG/Blueprints/Characters/Base/BP_UMCharacter_Base.HeadBone` _asbp_umcharacter_base))))
  ;[1 1 1] Try to deal melee damage on the server.
  (bind _output_get (set `local.LocalHit` UMHit))
  (bind (_bblockinghit _binitialoverlap _time _distance _location _impactpoint _normal _impactnormal _physmat _hitactor _hitcomponent _hitbonename _hititem _faceindex _tracestart) (`GameplayStatics.BreakHitResult` _output_get))
  (if _bblockinghit
    (set `local.LocalBone` _hitbonename)
    (set `local.LocalTraceStart` _tracestart)
    (set `local.LocalHitLocation` _location)
    (set `local.LocalActor` _hitactor)
    (`/Engine/EditorBlueprintResources/StandardMacros.IsValid` _physmat
      (:`Is Valid`
        (set `local.LocalSurfaceType` (`PhysicalMaterial.SurfaceType` _physmat)))
      (:`Is Not Valid`
        _))
    (if (`.DamageEnvironment?_58_7D6B7FF74E21EA991D03ECA8C68B7AFB` (break `/Game/UniversalMonster/Blueprints/Structs/S_TraceInfo` (`.Trace_131_8FC178054F11AD0076B3078EA6F165C7` (break `/Game/UniversalMonster/Blueprints/Structs/S_Attack` (`/Game/UniversalMonster/Blueprints/BP_UniversalMonster.Attack` (`/Game/UniversalMonster/Blueprints/BP_UMComponent.UniversalMonster` (`self.BP_UMComponent`)))))))
      ;;[1 1 1] Try to damage tree.
      (bind _asbp_instanced_component_tree_base (cast `/Game/EasySurvivalRPG/Blueprints/Components/InstancedComponents/BP_InstancedComponent_Tree_Base` _hitcomponent)
        (:`then`
          (`/Game/EasySurvivalRPG/Blueprints/Components/InstancedComponents/BP_InstancedComponent_Tree_Base.SpawnTree` _asbp_instanced_component_tree_base _hititem))
        (:`CastFailed`
          (bind _asbp_tree_base (cast `/Game/EasySurvivalRPG/Blueprints/InteractionObjects/Trees/BP_Tree_Base` (`local.LocalActor`))
            (:`then`
              (set `local.LocalTree` _asbp_tree_base)
              (`GameplayStatics.ApplyPointDamage` (`local.LocalActor`) _damage_3 (`local.LocalTraceStart`) (`local.LocalHit`) (`self.GetController`) self _damagetype_3)
              (`self.PlaySoundAtLocation (Multicast)` (`self.GetImpactSound` (`local.LocalSurfaceType`)) (`local.LocalHitLocation`)))
            (:`CastFailed`
              ;;[1 1 1] Try to damage mine.
              (bind _asbp_instanced_component_mine_base (cast `/Game/EasySurvivalRPG/Blueprints/Components/InstancedComponents/BP_InstancedComponent_Mine_Base` _hitcomponent)
                (:`then`
                  (`/Game/EasySurvivalRPG/Blueprints/Components/InstancedComponents/BP_InstancedComponent_Mine_Base.SpawnMine` _asbp_instanced_component_mine_base _hititem))
                (:`CastFailed`
                  (bind _asbp_mine_base (cast `/Game/EasySurvivalRPG/Blueprints/InteractionObjects/Mine/BP_Mine_Base` (`local.LocalActor`))
                    (:`then`
                      (set `local.LocalMine` _asbp_mine_base)
                      (`GameplayStatics.ApplyPointDamage` (`local.LocalActor`) _damage (`local.LocalTraceStart`) (`local.LocalHit`) (`self.GetController`) self _damagetype)
                      (`self.PlaySoundAtLocation (Multicast)` (`self.GetImpactSound` (`local.LocalSurfaceType`)) (`local.LocalHitLocation`)))
                    (:`CastFailed`
                      ;;[1 1 1] Try to deal damage to building or repair it if mallet is equiped.
                      (bind _asbp_building_building_object (cast `/Game/EasySurvivalRPG/Blueprints/InteractionObjects/BuildingObjects/Base/BP_Building_BuildingObject` (`local.LocalActor`))
                        (:`then`
                          (bind _asplayer_controller (cast `PlayerController` (`self.GetController`))
                            (:`then`
                              (bind _result (`/Game/EasySurvivalRPG/Blueprints/InteractionObjects/BuildingObjects/Base/BP_Building_BuildingObject.CheckOwnership` _asbp_building_building_object _asplayer_controller))
                              (if _result
                                (if (and _istool (`|EnumEquality` _tooltype "NewEnumerator3"))
                                  (`/Game/EasySurvivalRPG/Blueprints/InteractionObjects/BuildingObjects/Base/BP_Building_BuildingObject.Repair` _asbp_building_building_object _asplayer_controller)
                                  (else
                                    (`GameplayStatics.ApplyPointDamage` (`local.LocalActor`) _damage_4 (`local.LocalTraceStart`) (`local.LocalHit`) (`self.GetController`) self _damagetype_4 :!label _label)))
                                (else
                                  (goto _label))))
                            (:`CastFailed`
                              (goto _label)))
                          (`self.PlaySoundAtLocation (Multicast)` (`self.GetImpactSound` (`local.LocalSurfaceType`)) (`local.LocalHitLocation`)))
                        (:`CastFailed`
                          ;;[1 1 1] Try to damage character and other actors.
                          (bind _state (message `/Game/EasySurvivalRPG/Blueprints/Interfaces/BPI_Character.GetInteractionState_BPI` (`local.LocalActor`) "NewEnumerator3" :!label _label_2))
                          (if _state
                            (set `local.LocalSurfaceType` "SurfaceType3"))
                          (`GameplayStatics.ApplyPointDamage` (`local.LocalActor`) (select `bool` _returnvalue :`false` _damage_2 :`true` (* _damage_2 (select `bool` (`KismetArrayLibrary.Array_IsValidIndex` (`/Game/UniversalMonster/Blueprints/BP_UniversalMonster.Attacks` _universalmonster)) :`false` (`/Game/EasySurvivalRPG/Blueprints/Components/BP_AttributesComponent.GetAttributeValue` (`self.AttributesComponent`) (struct :`TagName` "EasyRPG.Attributes.Base.CriticalDamage")) :`true` (`.CritMultiplier_50_AA303BD84936FC24F5C7A9AB55416B81` (break `/Game/UniversalMonster/Blueprints/Structs/S_Attack` (`/Game/UniversalMonster/Blueprints/BP_UniversalMonster.Attack` _universalmonster)))))) (`local.LocalTraceStart`) (`local.LocalHit`) (`self.GetController`) self (select `bool` _returnvalue :`false` _damagetype_2 :`true` "/Game/EasySurvivalRPG/Blueprints/Misc/Other/BP_CriticalDamage.BP_CriticalDamage_C"))
                          (`self.PlaySoundAtLocation (Multicast)` (`self.GetImpactSound` (`local.LocalSurfaceType`)) (`local.LocalHitLocation`))
                          ;[1 1 1] Headshot
                          (if _returnvalue
                            (message `/Game/EasySurvivalRPG/Blueprints/Interfaces/BPI_Player.HeadshotNotification_BPI` self))))))))))))
      (else
        (goto _label_2)))))

(fn `UpdateTick`
  (params (DeltaSeconds :type "Float (double-precision)"))
  (returns (Success :type Boolean))
  (`self.UpdateStateWidgetRotation`)
  (`/Engine/EditorBlueprintResources/ActorMacros.Switch Has Authority`
    (:`Authority`
      (if (`self.IsAlive`)
        (if (< (`self.Health`) (`self.MaxHealth`))
          (`self.ChangeHealth` (* (`local.DeltaSeconds`) (`self.HealthRegeneration`))))
        (if (< (`self.Energy`) (`self.MaxEnergy`))
          (`self.ChangeEnergy` (* (`local.DeltaSeconds`) (`self.EnergyRegeneration`)))
          (return true)
          (else
            _))))
    (:`Remote`
      _))
  (return false))

(fn `UserConstructionScript`
  (bind _offhandmesh (`self.OffhandMesh`))
  (bind _weapon (`self.Weapon`))
  (`parent.UserConstructionScript`)
  (`ActorComponent.K2_DestroyComponent` (`self.AIPerception`))
  (`SceneComponent.K2_AttachToComponent` _weapon (`self.Mesh`) (`self.WeaponSocket`) "KeepRelative" "KeepRelative" "KeepRelative" true)
  (`SceneComponent.K2_SetRelativeTransform` _weapon (`self.WeaponTransform`) false false)
  (`SceneComponent.K2_AttachToComponent` _offhandmesh (`self.Mesh`) (`self.OffhandSocket`) "KeepRelative" "KeepRelative" "KeepRelative" true)
  (`SceneComponent.K2_SetRelativeTransform` _offhandmesh (`self.OffhandTransform`) false false)
  (`|ExecutionSequence`
    (:`then_0`
      (if (not (`self.bIsModular`))
        (`SceneComponent.SetVisibility` (`self.PantsMesh`) false false)
        (`SceneComponent.SetVisibility` (`self.HandsMesh`) false false)
        (`SceneComponent.SetVisibility` (`self.BodyMesh`) false false)
        (`SceneComponent.SetVisibility` (`self.HeadMesh`) false false)))
    (:`then_1`
      (if (not (`self.bShowWeapon`))
        (`SceneComponent.SetVisibility` (`self.WeaponMesh`) false false)))
    (:`then_2`
      (if (not (`self.bShowOffhand`))
        (`SceneComponent.SetVisibility` (`self.OffhandMesh`) false false)))))