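; Base character that bridges the Easy Survival RPG character to the Universal Monster system.
; On AI possession it enables AI and sets guard and patrol targets; lethal damage also toggles Universal Monster death.
; Enemy and threat checks combine saved faction relations with aggressive actors and current targets.
; Interface functions expose health, energy and weapon meshes, several others are stubs, and the tick's regeneration code is unreachable.
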(event `self.ReceivePossessed`
  (params (NewController :type "Controller Object Reference"))
  (bind _patrolpoint (`self.PatrolPoint`))
  (`parent.ReceivePossessed` NewController)
  (cast `/Game/UniversalMonster/AI/AIC_UniversalMonster` NewController)
  (`KismetSystemLibrary.Delay` 0.1)
  (`self.EnableAI`)
  (`self.SetGuardLocation` (`self.GuardLocation`))
  (`/Engine/EditorBlueprintResources/StandardMacros.IsValid` _patrolpoint
    (:`Is Valid`
      (`self.SetPatrolPoint` _patrolpoint))))

(event `self.ReceiveDestroyed`
  (bind _asbp_character_undead (cast `/Game/EasySurvivalRPG/Blueprints/Characters/Base/BP_Character_Undead` self)
    (:`then`
      (`/Game/EasySurvivalRPG/Blueprints/Characters/Base/BP_Character_Undead.DeleteMark (Multicast)` _asbp_character_undead)
      (`self.SetLifeSpan` (`/Game/EasySurvivalRPG/Blueprints/Components/BP_FoliageCheckerComponent.FoliageChecker` (`/Game/EasySurvivalRPG/Blueprints/Characters/Base/BP_Character_Undead.FoliageCheckerComponent` _asbp_character_undead)) 0.01))
    (:`CastFailed`
      _))
  (`parent.ReceiveDestroyed`))

(fn `ChangeHealth`
  (params (Value :type "Float (double-precision)") (Percent :type Boolean) (InstigatedBy :type "Controller Object Reference"))
  (returns (Success :type Boolean))
  ;[1 1 1] Change health value.
  (if (`self.IsAlive`)
    (bind _output_get (set `self.Health` (`KismetMathLibrary.FClamp` (+ (select `bool` Percent :`false` Value :`true` (* Value (`self.MaxHealth`))) (`self.Health`)) 0.0 (`self.MaxHealth`))))
    (if (<= _output_get 0.0)
      (`self.Death` (`local.InstigatedBy`))
      (`/Game/UniversalMonster/Blueprints/BP_UniversalMonster.ToggleDeath` (`/Game/UniversalMonster/Blueprints/BP_UMComponent.UniversalMonster` (`self.BP_UMComponent`)) true)))
  (return true))

(fn `GetBulletInfo`
  (returns (BulletInfo :type "/Game/UniversalMonster/Blueprints/Structs/S_BulletInfo Structure"))
  (return))

(fn `GetSlotName`
  (returns (SlotName :type String))
  (bind _asbp_game_instance (cast `/Game/EasySurvivalRPG/Blueprints/Game/GameInstance/BP_GameInstance` (`GameplayStatics.GetGameInstance`))
    (:`then`
      (bind _currentgamesave (`/Game/EasySurvivalRPG/Blueprints/Game/GameInstance/BP_GameInstance.CurrentGameSave` _asbp_game_instance)
        (:`then`
          (return (`/Game/EasySurvivalRPG/Blueprints/Game/GameSaves/BP_GameSave_Session.SlotName` _currentgamesave)))
        (:`else`
          _)))
    (:`CastFailed`
      _))
  (return ""))

(fn `GetStat`
  (params (Stat :type "/Game/UniversalMonster/Blueprints/Enums/E_StatName Enum" :default "NewEnumerator0"))
  (returns (Value :type "Float (double-precision)"))
  (bind _health (`self.Health`))
  (bind _maxhealth (`self.MaxHealth`))
  (bind _energy (`self.Energy`))
  (bind _maxenergy (`self.MaxEnergy`))
  (return (select `/Game/UniversalMonster/Blueprints/Enums/E_StatName` Stat :`NewEnumerator0` _health :`NewEnumerator8` _maxhealth :`NewEnumerator1` (/ _health _maxhealth) :`NewEnumerator2` _energy :`NewEnumerator9` _maxenergy :`NewEnumerator3` (/ _energy _maxenergy))))

(fn `GetUM`
  (returns (UniversalMonster :type "/Game/UniversalMonster/Blueprints/BP_UniversalMonster Object Reference"))
  (return null))

(fn `GetWeaponMesh`
  (params (SocketName :type Name))
  (returns (StaticMesh :type "StaticMesh Object Reference"))
  (for _array_element (`self.GetAttachedActors` true)
    (bind _asbp_usable_item_base (cast `/Game/EasySurvivalRPG/Blueprints/InteractionObjects/UsableItems/Base/BP_UsableItem_Base` _array_element))
    (if (== (`self.GetAttachParentSocketName` _asbp_usable_item_base) (`local.SocketName`))
      (return (`/Game/EasySurvivalRPG/Blueprints/InteractionObjects/UsableItems/Base/BP_UsableItem_Base.StaticMesh` _asbp_usable_item_base))))
  (bind _asbp_umcharacter_player (cast `/Game/EasySurvivalRPG/Blueprints/Characters/Base/BP_UMCharacter_Player` self)
    (:`then`
      (if (== (`/Game/EasySurvivalRPG/Blueprints/Characters/Base/BP_UMCharacter_Base.OffhandSocket` _asbp_umcharacter_player) (`local.SocketName`))
        (return (`StaticMeshComponent.StaticMesh` (`/Game/EasySurvivalRPG/Blueprints/Characters/Base/BP_UMCharacter_Player.OffhandMesh` _asbp_umcharacter_player)))))
    (:`CastFailed`
      (bind _asbp_umcharacter_enemy (cast `/Game/EasySurvivalRPG/Blueprints/Characters/Base/BP_UMCharacter_Enemy` self)
        (:`then`
          (if (== (`/Game/EasySurvivalRPG/Blueprints/Characters/Base/BP_UMCharacter_Base.OffhandSocket` _asbp_umcharacter_enemy) (`local.SocketName`))
            (return (`StaticMeshComponent.StaticMesh` (`/Game/EasySurvivalRPG/Blueprints/Characters/Base/BP_UMCharacter_Enemy.OffhandMesh` _asbp_umcharacter_enemy)))))
        (:`CastFailed`
          (return null))))))

(fn `HitEffect`
  (params (Hit :type "HitResult Structure") (Effect :type "/Game/UniversalMonster/Blueprints/Structs/S_HitEffect Structure"))
  (returns (`bResult?` :type Boolean))
  (return false))

(fn `SetStat`
  (params (Stat :type "/Game/UniversalMonster/Blueprints/Enums/E_StatName Enum" :default "NewEnumerator0") (Value :type "Float (double-precision)"))
  (returns (`bResult?` :type Boolean))
  (switch `/Game/UniversalMonster/Blueprints/Enums/E_StatName` Stat
    (:`NewEnumerator0`
      (set `self.Health` Value))
    (:`NewEnumerator8`
      (set `self.MaxHealth` Value))
    (:`NewEnumerator1`
      (return false))
    (:`NewEnumerator2`
      (set `self.Energy` Value))
    (:`NewEnumerator9`
      (set `self.MaxEnergy` Value))
    (:`NewEnumerator3`
      (return false))
    (:`NewEnumerator4`
      (return false))
    (:`NewEnumerator10`
      (return false))
    (:`NewEnumerator5`
      (return false))
    (:`NewEnumerator6`
      (return false))
    (:`NewEnumerator11`
      (return false))
    (:`NewEnumerator7`
      (return false))
    (:`NewEnumerator12`
      (return false))
    (:`NewEnumerator13`
      (return false))
    (:`NewEnumerator14`
      (return false)))
  (return true))

(fn `TargetIsEnemy`
  (params (Target :type "Actor Object Reference"))
  (returns (IsEnemy :type Boolean))
  (locals (TargetUM :type "/Game/UniversalMonster/Blueprints/BP_UniversalMonster Object Reference"))
  (bind _universalmonster (`/Game/UniversalMonster/Blueprints/BP_UMComponent.UniversalMonster` (`self.BP_UMComponent`)))
  (bind _returnvalue (or (`KismetArrayLibrary.Array_Contains` (`self.AggressiveActors`) Target) (== Target (`self.TargetActor`)) (== Target (`/Game/UniversalMonster/Blueprints/BP_UniversalMonster.CurrentTarget` (`/Game/UniversalMonster/Blueprints/BP_UMComponent.UniversalMonster` (`self.BP_UMComponent`))))))
  ;[1 1 1] Returns true if target actor is enemy.
  (bind _output_get (set `local.TargetUM` (`/Game/UniversalMonster/Blueprints/BPFL_UMFunctions.GetUniversalMonster` Target)))
  (`/Engine/EditorBlueprintResources/StandardMacros.IsValid` _output_get
    (:`Is Valid`
      (return (or (`KismetArrayLibrary.Array_Contains` (`|MakeArray` "NewEnumerator7" "NewEnumerator2" "NewEnumerator8" :!type "/Game/UniversalMonster/Blueprints/Enums/E_FactionState Enum") (`/Game/UniversalMonster/Blueprints/BP_UMSaveGame.GetFactionState` (`/Game/UniversalMonster/Blueprints/BP_UMGlobal.UMSaveGame` (`/Game/UniversalMonster/Blueprints/BP_UniversalMonster.UMGlobal` _universalmonster)) (`.RowName` (break `DataTableRowHandle` (`/Game/UniversalMonster/Blueprints/BP_UniversalMonster.Faction` _universalmonster))) (`.RowName` (break `DataTableRowHandle` (`/Game/UniversalMonster/Blueprints/BP_UniversalMonster.Faction` _output_get))))) _returnvalue)))
    (:`Is Not Valid`
      (if (`KismetSystemLibrary.DoesImplementInterface` Target "/Game/EasySurvivalRPG/Blueprints/Interfaces/BPI_Character.BPI_Character_C")
        (message `/Game/EasySurvivalRPG/Blueprints/Interfaces/BPI_Character.GetFraction_BPI` Target)
        (return (or false _returnvalue))
        (else
          (return false))))))

(fn `TargetIsThreat`
  (params (Target :type "Actor Object Reference (by ref)"))
  (returns (IsThreat :type Boolean))
  (locals (TargetUM :type "/Game/UniversalMonster/Blueprints/BP_UniversalMonster Object Reference"))
  (bind _returnvalue (`KismetArrayLibrary.Array_Contains` (`self.AggressiveActors`) Target))
  (bind _universalmonster (`/Game/UniversalMonster/Blueprints/BP_UMComponent.UniversalMonster` (`self.BP_UMComponent`)))
  ;[1 1 1] Returns true if target actor is threat.
  (bind _output_get (set `local.TargetUM` (`/Game/UniversalMonster/Blueprints/BPFL_UMFunctions.GetUniversalMonster` Target)))
  (`/Engine/EditorBlueprintResources/StandardMacros.IsValid` _output_get
    (:`Is Valid`
      (return (or (not (`KismetArrayLibrary.Array_Contains` (`|MakeArray` "NewEnumerator3" "NewEnumerator4" "NewEnumerator5" "NewEnumerator0" "NewEnumerator1" :!type "/Game/UniversalMonster/Blueprints/Enums/E_FactionState Enum") (`/Game/UniversalMonster/Blueprints/BP_UMSaveGame.GetFactionState` (`/Game/UniversalMonster/Blueprints/BP_UMGlobal.UMSaveGame` (`/Game/UniversalMonster/Blueprints/BP_UniversalMonster.UMGlobal` _universalmonster)) (`.RowName` (break `DataTableRowHandle` (`/Game/UniversalMonster/Blueprints/BP_UniversalMonster.Faction` _universalmonster))) (`.RowName` (break `DataTableRowHandle` (`/Game/UniversalMonster/Blueprints/BP_UniversalMonster.Faction` _output_get)))))) _returnvalue (== Target (`self.TargetActor`)))))
    (:`Is Not Valid`
      (if (`KismetSystemLibrary.DoesImplementInterface` Target "/Game/EasySurvivalRPG/Blueprints/Interfaces/BPI_Character.BPI_Character_C")
        (message `/Game/EasySurvivalRPG/Blueprints/Interfaces/BPI_Character.GetFraction_BPI` Target)
        (return (or (not false) _returnvalue))
        (else
          (return false))))))

(fn `TaskEvent`
  (params (Task :type "/Game/UniversalMonster/Blueprints/Structs/S_Task Structure"))
  (returns (`bResult?` :type Boolean))
  (return false))

(fn `UMHit`
  (params (UniversalMonster :type "/Game/UniversalMonster/Blueprints/BP_UniversalMonster Object Reference") (Attack :type "/Game/UniversalMonster/Blueprints/Structs/S_Attack Structure") (HitBox :type "BoxComponent Object Reference") (Projectile :type "/Game/UniversalMonster/Blueprints/BP_UMProjectile Object Reference") (Timer :type "/Game/UniversalMonster/Blueprints/BP_UMTimer Object Reference") (Bullet :type "/Game/UniversalMonster/Blueprints/Structs/S_BulletInfo Structure") (Hit :type "HitResult Structure"))
  (returns (`bResult?` :type Boolean))
  (return true))

(fn `UpdateTick`
  (params (DeltaSeconds :type "Float (double-precision)"))
  (returns (Success :type Boolean))
  ;[1 1 1] Update character's state by tick.
  (bind _success (`parent.UpdateTick` DeltaSeconds))
  (return _success))

(fn `UserConstructionScript`
  (`parent.UserConstructionScript`))