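; Function library for the Universal Monster system, providing shared helpers for monster decisions and attack resolution.
; CheckAllConditions gates on stimulus and self/target stat comparisons, accepting non-monster targets only if their instigator is player-controlled.
; Other helpers measure radius-adjusted distance, resolve monsters via cast or component, and roll crit-weighted damage.
; ShouldHit filters hits by ignored classes, repeats and environment settings; its alive and faction friendly-fire checks are unconnected.
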(fn `CheckAllConditions`
  (params (TargetActor :type "Actor Object Reference") (SelfActor :type "Actor Object Reference") (StimulusConditions :type "Array of /Game/UniversalMonster/Blueprints/Structs/S_StimulusCondition Structure (by ref)") (StimulusInfo :type "/Game/UniversalMonster/Blueprints/Structs/S_StimulusInfo Structure") (SelfConditions :type "Array of /Game/UniversalMonster/Blueprints/Structs/S_StatCondition Structure (by ref)") (TargetConditions :type "Array of /Game/UniversalMonster/Blueprints/Structs/S_StatCondition Structure (by ref)") (ErrorTolerance :type "Float (double-precision)" :default 0.0001))
  (returns (`bSuccess?` :type Boolean))
  (bind _universalmonster (`self.GetUniversalMonster` TargetActor TargetActor))
  (bind _bsuccess_ (`self.CheckStimulus` SelfActor StimulusConditions ErrorTolerance StimulusInfo SelfActor))
  (if _bsuccess_
    (bind _bsuccess__2 (`self.CheckStats` SelfActor SelfConditions ErrorTolerance SelfActor))
    (if _bsuccess__2
      (`/Engine/EditorBlueprintResources/StandardMacros.IsValid` TargetActor
        (:`Is Valid`
          (`/Engine/EditorBlueprintResources/StandardMacros.IsValid` _universalmonster
            (:`Is Valid`
              (bind _bsuccess__3 (`self.CheckStats` _universalmonster TargetConditions ErrorTolerance _universalmonster))
              (if _bsuccess__3
                (return true)
                (else
                  _)))
            (:`Is Not Valid`
              (if (`Pawn.IsPlayerControlled` (`Actor.Instigator` TargetActor))
                (return true)
                (else
                  _)))))
        (:`Is Not Valid`
          _))))
  (return false))

(fn `CheckStats`
  (params (Actor :type "Actor Object Reference") (`Stat Conditions` :type "Array of /Game/UniversalMonster/Blueprints/Structs/S_StatCondition Structure") (`Error Tolerance` :type "Float (double-precision)"))
  (returns (`bSuccess?` :type Boolean))
  (if (`KismetSystemLibrary.DoesImplementInterface` Actor "/Game/UniversalMonster/Blueprints/BPI_UniversalMonster.BPI_UniversalMonster_C")
    (for _array_element `Stat Conditions`
      (bind _value (message `/Game/UniversalMonster/Blueprints/BPI_UniversalMonster.GetStat` Actor (break `/Game/UniversalMonster/Blueprints/Structs/S_StatCondition` _array_element)))
      (if (not (`self.CompareValues` _value (`.Condition_7_922E61734BDDED4EE0F081BB39CB3EDF` (break `/Game/UniversalMonster/Blueprints/Structs/S_StatCondition` _array_element)) (`.Value_6_9464E87743A1789ECE567EBB9168E01E` (break `/Game/UniversalMonster/Blueprints/Structs/S_StatCondition` _array_element)) `Error Tolerance` Actor))
        (return false)))
    (return true)
    (else
      (return true))))

(fn `CheckStimulus`
  (params (Actor :type "Actor Object Reference") (StimulusConditions :type "Array of /Game/UniversalMonster/Blueprints/Structs/S_StimulusCondition Structure") (ErrorTolerance :type "Float (double-precision)") (StimulusInfo :type "/Game/UniversalMonster/Blueprints/Structs/S_StimulusInfo Structure"))
  (returns (`bSuccess?` :type Boolean))
  (for _array_element StimulusConditions
    (if (not (`self.CompareValues` (select `/Game/UniversalMonster/Blueprints/Enums/E_StimulusInfo` (break `/Game/UniversalMonster/Blueprints/Structs/S_StimulusCondition` _array_element) :`NewEnumerator4` StimulusInfo_Age_2_429E572A440DCDAA85FC09A8A8DA3CFC :`NewEnumerator5` StimulusInfo_Expiration_12_DBDE1F6F409E80D1CCD7C09E46E7CF19 :`NewEnumerator6` StimulusInfo_Strength_13_850E30F945F323DBD5EA37B5AD58E535 :`NewEnumerator7` StimulusInfo_Distance_14_1A4C44CC442A0D21B4C65AB09C4FC5E3 :`NewEnumerator9` StimulusInfo_StimulusX_15_D57AB6364687FBC5E182DEB3E6C29316 :`NewEnumerator10` StimulusInfo_StimulusY_16_DA9A36E34F40977019335F87DA29568F :`NewEnumerator11` StimulusInfo_StimulusZ_17_4A8AECAE42781DDA3070A2BE652A5DC7 :`NewEnumerator12` StimulusInfo_ReceiverX_18_C8AF53914EEA6297E9F6FE8700E8EB71 :`NewEnumerator13` StimulusInfo_ReceiverY_19_52BEC7884D95004D5AE2F19984C92524 :`NewEnumerator14` StimulusInfo_ReceiverZ_20_F797DBDE4B67601932D011970816CF25 :`NewEnumerator16` (`KismetMathLibrary.Conv_BoolToDouble` `StimulusInfo_LineOfSight?_34_DBFBB5F542E5B6998EDBEC844406EA8A`) :`NewEnumerator17` (`KismetMathLibrary.Conv_BoolToDouble` `StimulusInfo_InAttackRange?_30_B3779AEF40843C42067C38AD8AEA7676`) :`NewEnumerator22` (`KismetMathLibrary.Conv_BoolToDouble` `StimulusInfo_TargetAttacking?_42_C75B5FDD4176A2C6EC2FE292809D445E`) :`NewEnumerator15` StimulusInfo_DistanceFromSpawn_33_19A1C75E480F612832292DAF40C8CE36 :`NewEnumerator19` StimulusInfo_ForwardDotProduct_36_C89F55D947796B0695BD3E909F88040F :`NewEnumerator20` StimulusInfo_RightDotProduct_38_F7C9D413447497A79DB27E83A8812CFD :`NewEnumerator21` StimulusInfo_UpDotProduct_40_509DA9574F300E5A99AEAABAE5E8F614) (`.Condition_7_922E61734BDDED4EE0F081BB39CB3EDF` (break `/Game/UniversalMonster/Blueprints/Structs/S_StimulusCondition` _array_element)) (`.Value_6_9464E87743A1789ECE567EBB9168E01E` (break `/Game/UniversalMonster/Blueprints/Structs/S_StimulusCondition` _array_element)) ErrorTolerance Actor))
      (return false)))
  (return true))

(fn `CompareValues`
  (params (`Value 1` :type "Float (double-precision)") (Condition :type "/Game/UniversalMonster/Blueprints/Enums/E_Conditional Enum" :default "NewEnumerator0") (`Value 2` :type "Float (double-precision)") (`Error Tolerance` :type "Float (double-precision)"))
  (returns (Result :type Boolean))
  (return (select `/Game/UniversalMonster/Blueprints/Enums/E_Conditional` Condition :`NewEnumerator0` (< `Value 1` `Value 2`) :`NewEnumerator1` (<= `Value 1` `Value 2`) :`NewEnumerator2` (select `bool` (> `Error Tolerance` 0.0) :`false` (== `Value 1` `Value 2`) :`true` (`KismetMathLibrary.NearlyEqual_FloatFloat` `Value 1` `Value 2` `Error Tolerance`)) :`NewEnumerator3` (!= `Value 1` `Value 2`) :`NewEnumerator4` (>= `Value 1` `Value 2`) :`NewEnumerator5` (> `Value 1` `Value 2`))))

(fn `DistanceBetweenActors`
  (params (From :type "Actor Object Reference") (To :type "Actor Object Reference"))
  (returns (Distance :type "Float (double-precision)"))
  (return (- (- (`Actor.GetHorizontalDistanceTo` From To) (`self.GetActorRadius` From From)) (`self.GetActorRadius` To From))))

(fn `GetActorRadius`
  (params (Actor :type "Actor Object Reference"))
  (returns (Radius :type "Float (double-precision)"))
  (bind (_origin _boxextent) (`Actor.GetActorBounds` Actor true false))
  (`/Engine/EditorBlueprintResources/StandardMacros.IsValid` Actor
    (:`Is Valid`
      (bind _ascharacter (cast `Character` Actor)
        (:`then`
          (return (`CapsuleComponent.GetScaledCapsuleRadius` (`Character.CapsuleComponent` _ascharacter))))
        (:`CastFailed`
          (return (/ (`KismetMathLibrary.FMin` (.x _boxextent) (.y _boxextent)) 2.0)))))
    (:`Is Not Valid`
      (return -1.0))))

(fn `GetDamage`
  (params (Attack :type "/Game/UniversalMonster/Blueprints/Structs/S_Attack Structure (by ref)"))
  (returns (Damage :type "Float (double-precision)"))
  (bind ((`MinDamage_29_F81766C343A65D750068C9BE3944D6E3` _mindamage) (`MaxDamage_30_F6C1C2F747F381BA64BCABB31229A7DB` _maxdamage) (`CritChance_49_D8D544FA492ECA9A154C558913491C70` _critchance) (`CritMultiplier_50_AA303BD84936FC24F5C7A9AB55416B81` _critmultiplier)) (break `/Game/UniversalMonster/Blueprints/Structs/S_Attack` Attack))
  (return (* (`KismetMathLibrary.RandomFloatInRange` _mindamage _maxdamage) (select `bool` (`KismetMathLibrary.RandomBoolWithWeight` _critchance) :`false` 1.0 :`true` _critmultiplier))))

(fn `GetUMComponent`
  (params (Actor :type "Actor Object Reference"))
  (returns (UMComponent :type "/Game/UniversalMonster/Blueprints/BP_UMComponent Object Reference"))
  (return (`Actor.GetComponentByClass` Actor "/Game/UniversalMonster/Blueprints/BP_UMComponent.BP_UMComponent_C")))

(fn `GetUniversalMonster`
  (params (Actor :type "Actor Object Reference"))
  (returns (UniversalMonster :type "/Game/UniversalMonster/Blueprints/BP_UniversalMonster Object Reference"))
  (bind _returnvalue (`Actor.GetComponentByClass` Actor "/Game/UniversalMonster/Blueprints/BP_UMComponent.BP_UMComponent_C"))
  (bind _asbp_universal_monster (cast `/Game/UniversalMonster/Blueprints/BP_UniversalMonster` Actor)
    (:`then`
      (return _asbp_universal_monster))
    (:`CastFailed`
      (`/Engine/EditorBlueprintResources/StandardMacros.IsValid` Actor
        (:`Is Valid`
          (`/Engine/EditorBlueprintResources/StandardMacros.IsValid` _returnvalue
            (:`Is Valid`
              (return (`/Game/UniversalMonster/Blueprints/BP_UMComponent.UniversalMonster` _returnvalue)))
            (:`Is Not Valid`
              (return null))))
        (:`Is Not Valid`
          (return null))))))

(fn `IsAlive`
  (params (Actor :type "Actor Object Reference (by ref)"))
  (returns (ReturnValue :type Boolean))
  (if (`KismetSystemLibrary.DoesImplementInterface` Actor "/Game/UniversalMonster/Blueprints/BPI_UniversalMonster.BPI_UniversalMonster_C")
    (bind _value (message `/Game/UniversalMonster/Blueprints/BPI_UniversalMonster.GetStat` Actor "NewEnumerator0"))
    (return (> _value 0.0))
    (else
      (return true))))

(fn `ShouldHit`
  (params (Hit :type "HitResult Structure") (Attack :type "/Game/UniversalMonster/Blueprints/Structs/S_Attack Structure (by ref)") (UM :type "/Game/UniversalMonster/Blueprints/BP_UniversalMonster Object Reference") (HitActors :type "Array of Actor Object Reference (by ref)"))
  (returns (`ShouldHit?` :type Boolean) (`ShouldPassThrough?` :type Boolean) (HitActor :type "Actor Object Reference"))
  (locals (Actor :type "Actor Object Reference") (Component :type "PrimitiveComponent Object Reference") (HitUM :type "/Game/UniversalMonster/Blueprints/BP_UniversalMonster Object Reference") (PassThrough :type Boolean :default false))
  (bind (_bblockinghit _binitialoverlap _time _distance _location _impactpoint _normal _impactnormal _physmat _hitactor _hitcomponent) (`GameplayStatics.BreakHitResult` Hit))
  (bind _actor (`local.Actor`))
  (bind ((`PassThroughEnvironment?_57_4C6AB1614244EEF06847E594530030D2` _passthroughenvironment_) (`DamageEnvironment?_58_7D6B7FF74E21EA991D03ECA8C68B7AFB` _damageenvironment_) (`EnvironmentObjects_68_114C2B3A46F5CCCC4ABFC3B2F31EE033` _environmentobjects)) (break `/Game/UniversalMonster/Blueprints/Structs/S_TraceInfo` (`.Trace_131_8FC178054F11AD0076B3078EA6F165C7` (break `/Game/UniversalMonster/Blueprints/Structs/S_Attack` (`local.Attack`)))))
  (if _bblockinghit
    (set `local.Actor` _hitactor)
    (set `local.Component` _hitcomponent)
    (if (`self.ShouldIgnore` (`local.Attack`) _actor (`local.Component`) _actor)
      _
      (elif (and (`.OneHitPerActor?_40_0120D9244E9E912FC3F525B9AFF42611` (break `/Game/UniversalMonster/Blueprints/Structs/S_TraceInfo` (`.Trace_131_8FC178054F11AD0076B3078EA6F165C7` (break `/Game/UniversalMonster/Blueprints/Structs/S_Attack` (`local.Attack`))))) (`KismetArrayLibrary.Array_Contains` (`local.HitActors`) (`local.Actor`)))
        _
        (elif (`KismetArrayLibrary.Array_Contains` _environmentobjects (`PrimitiveComponent.GetCollisionObjectType` (`local.Component`)))
          (if _damageenvironment_
            (set `local.PassThrough` _passthroughenvironment_)
            (return true (`local.PassThrough`) (`local.Actor`))
            (else
              _))
          (else
            (set `local.PassThrough` (`.PassThroughFriends?_51_ED15E1504E2EB62D3C5CF58FACD2E1DD` (break `/Game/UniversalMonster/Blueprints/Structs/S_TraceInfo` (`.Trace_131_8FC178054F11AD0076B3078EA6F165C7` (break `/Game/UniversalMonster/Blueprints/Structs/S_Attack` (`local.Attack`))))))
            (return true (`local.PassThrough`) (`local.Actor`)))))))
  (return false (`local.PassThrough`) null))

(fn `ShouldIgnore`
  (params (Attack :type "/Game/UniversalMonster/Blueprints/Structs/S_Attack Structure (by ref)") (Actor :type "Actor Object Reference (by ref)") (Component :type "PrimitiveComponent Object Reference"))
  (returns (ReturnValue :type Boolean))
  (bind ((`ClassesToIgnore_41_6AD09E77430CC95B8B8EECAC1E71CC2B` _classestoignore)) (break `/Game/UniversalMonster/Blueprints/Structs/S_TraceInfo` (`.Trace_131_8FC178054F11AD0076B3078EA6F165C7` (break `/Game/UniversalMonster/Blueprints/Structs/S_Attack` Attack))))
  (return (or (`KismetArrayLibrary.Array_Contains` _classestoignore (`GameplayStatics.GetObjectClass` Actor)) (`KismetArrayLibrary.Array_Contains` _classestoignore (`GameplayStatics.GetObjectClass` Component)))))