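; BP_UMGlobal is a component that manages the Universal Monster save game and its faction data.
; On construction, it derives the slot name from its owner plus a "_UM" suffix, keeping its default if none is supplied.
; BeginPlay loads BP_UMSaveGame or creates one initialized from FactionsDT.
; Loaded saves reconcile only when faction counts differ, appending tail rows by index or removing factions missing from the table.
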(event `self.ReceiveBeginPlay`
  (bind _returnvalue (`GameplayStatics.LoadGameFromSlot` (`self.SlotName`)))
  (bind _asbp_umsave_game (cast `/Game/UniversalMonster/Blueprints/BP_UMSaveGame` _returnvalue)
    (:`then`
      (set `self.UMSaveGame` _asbp_umsave_game)
      (`self.CheckFactionData`))
    (:`CastFailed`
      (bind _returnvalue_2 (`GameplayStatics.CreateSaveGameObject` "/Game/UniversalMonster/Blueprints/BP_UMSaveGame.BP_UMSaveGame_C"))
      (bind _output_get (set `self.UMSaveGame` _returnvalue_2))
      (set `/Game/UniversalMonster/Blueprints/BP_UMSaveGame.SlotName` (`self.SlotName`) _output_get)
      (`/Game/UniversalMonster/Blueprints/BP_UMSaveGame.InitializeFactions` _output_get (`self.FactionsDT`)))))

(fn `CheckFactionData`
  (locals (FactionRows :type "Array of Name"))
  (bind _returnvalue (`KismetArrayLibrary.Array_Length` (`/Game/UniversalMonster/Blueprints/BP_UMSaveGame.Factions` (`self.UMSaveGame`))))
  (bind _outrownames (`DataTableFunctionLibrary.GetDataTableRowNames` (`self.FactionsDT`)))
  (set `local.FactionRows` _outrownames)
  (bind _returnvalue_2 (`KismetArrayLibrary.Array_Length` _outrownames))
  (if (> _returnvalue_2 _returnvalue)
    (for _index (range _returnvalue _returnvalue_2)
      (bind _returnvalue_3 (`|GetDataTableRow` (`self.FactionsDT`) (`|GetArrayItem` (`local.FactionRows`) _index))
        (:`then`
          (`/Game/UniversalMonster/Blueprints/BP_UMSaveGame.AddFaction` (`self.UMSaveGame`) _returnvalue_3))))
    (elif (< _returnvalue_2 _returnvalue)
      (bind (_arrayindex _arrayelement) (`/Engine/EditorBlueprintResources/StandardMacros.ReverseForEachLoop` (`/Game/UniversalMonster/Blueprints/BP_UMSaveGame.Factions` (`self.UMSaveGame`)))
        (:`LoopBody`
          (bind ((`FactionName_20_BA658D3A40F60942823D75BB3D79ABE7` _factionname)) (break `/Game/UniversalMonster/Blueprints/Structs/S_Faction` _arrayelement))
          (if (not (`KismetArrayLibrary.Array_Contains` (`local.FactionRows`) _factionname))
            (`/Game/UniversalMonster/Blueprints/BP_UMSaveGame.RemoveFaction` (`self.UMSaveGame`) _factionname)))))))

(fn `UserConstructionScript`
  (bind _slotname (message `/Game/UniversalMonster/Blueprints/BPI_UniversalMonster.GetSlotName` (`self.GetOwner`)))
  (set `self.SlotName` (`KismetMathLibrary.SelectString` (`KismetStringLibrary.Concat_StrStr` _slotname "_UM") (`self.SlotName`) (`KismetStringLibrary.NotEqual_StrStr` _slotname))))