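; SaveGame object for Universal Monster that persists factions, their mutual reputations and a stats list, seeded from DataTables when empty.
; Each faction holds a reputation array indexed like the Factions list, so adding or removing a faction resizes every array to keep the matrix aligned.
; A GetFaction macro resolves names for lookups and edits, and GetFactionState maps reputation thresholds to enum tiers.
; Mutating functions save to the slot immediately.
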(fn `AddFaction`
  (params (Faction :type "/Game/UniversalMonster/Blueprints/Structs/S_Faction Structure"))
  (locals (LocalReputations :type "Array of Float (double-precision)"))
  (bind ((`FactionName_20_BA658D3A40F60942823D75BB3D79ABE7` _factionname) (`Reputations_16_A7D8009747F1AD4E22A5A4B295B4667E` _reputations)) (break `/Game/UniversalMonster/Blueprints/Structs/S_Faction` Faction))
  (bind _factions (`self.Factions`))
  (bind _localreputations (`local.LocalReputations`))
  (bind ((`FactionName_20_BA658D3A40F60942823D75BB3D79ABE7` _factionname_2) (`IsPlayerFaction?_11_CBBAFD194560C4701829DAAD4DD6A629` _isplayerfaction_) (`DefaultReputation_23_41C400BF443B9E32D1111BB984C72371` _defaultreputation)) (break `/Game/UniversalMonster/Blueprints/Structs/S_Faction` (`local.Faction`)))
  (`self.GetFaction` _factionname
    (:`NotFound`
      (set `local.LocalReputations` _reputations)
      (for (_ _array_index) _factions
        (bind ((`Reputations_16_A7D8009747F1AD4E22A5A4B295B4667E` _reputations_2) (`DefaultReputation_23_41C400BF443B9E32D1111BB984C72371` _defaultreputation_2)) (break `/Game/UniversalMonster/Blueprints/Structs/S_Faction` (`|GetArrayItem` (`self.Factions`) _array_index)))
        (`KismetArrayLibrary.Array_Add` _reputations_2 _defaultreputation_2)
        (if (< (`KismetArrayLibrary.Array_LastIndex` (`local.LocalReputations`)) _array_index)
          (`KismetArrayLibrary.Array_Add` (`local.LocalReputations`) _defaultreputation)))
      (if (== (`KismetArrayLibrary.Array_Length` _factions) (`KismetArrayLibrary.Array_Length` (`local.LocalReputations`)))
        (`KismetArrayLibrary.Array_Add` _localreputations 4.0))
      (`KismetArrayLibrary.Array_AddUnique` (`self.Factions`) (make `/Game/UniversalMonster/Blueprints/Structs/S_Faction` _factionname_2 _isplayerfaction_ _localreputations _defaultreputation))
      (`GameplayStatics.SaveGameToSlot` self (`self.SlotName`)))))

(fn `AddReputation`
  (params (`Faction Name` :type Name) (`Target Faction` :type Name) (Amount :type "Float (double-precision)"))
  (locals (FactionIndex :type Integer :default 0) (TargetIndex :type Integer :default 0))
  (bind _faction (`self.GetFaction` `Faction Name`)
    (:`Found`
      (bind (_faction_2 _index) (`self.GetFaction` `Target Faction`)
        (:`Found`
          (set `local.TargetIndex` _index)
          (bind ((`Reputations_16_A7D8009747F1AD4E22A5A4B295B4667E` _reputations)) (break `/Game/UniversalMonster/Blueprints/Structs/S_Faction` _faction))
          (`KismetArrayLibrary.Array_Set` _reputations (`local.TargetIndex`) (+ (`|GetArrayItem` _reputations (`local.TargetIndex`)) Amount))
          (`GameplayStatics.SaveGameToSlot` self (`self.SlotName`)))))))

(fn `FindFaction`
  (params (FactionName :type Name))
  (returns (Faction :type "/Game/UniversalMonster/Blueprints/Structs/S_Faction Structure (by ref)") (Index :type Integer))
  (bind (_faction _index) (`self.GetFaction` FactionName)
    (:`Found`
      (return _faction _index))
    (:`NotFound`
      (return (struct) -1))))

(fn `GetFactionState`
  (params (FactionName :type Name) (TargetFaction :type Name))
  (returns (FactionState :type "/Game/UniversalMonster/Blueprints/Enums/E_FactionState Enum"))
  (bind _reputation (`self.GetReputation` FactionName TargetFaction))
  (return (select `bool` (<= _reputation -4.0) :`false` (select `bool` (<= _reputation -3.0) :`false` (select `bool` (<= _reputation -2.0) :`false` (select `bool` (<= _reputation -1.0) :`false` (select `bool` (< _reputation 1.0) :`false` (select `bool` (< _reputation 2.0) :`false` (select `bool` (< _reputation 3.0) :`false` (select `bool` (< _reputation 4.0) :`false` "NewEnumerator3" :`true` "NewEnumerator4" :!type "/Game/UniversalMonster/Blueprints/Enums/E_FactionState Enum") :`true` "NewEnumerator5") :`true` "NewEnumerator0") :`true` "NewEnumerator1") :`true` "NewEnumerator6") :`true` "NewEnumerator8") :`true` "NewEnumerator2") :`true` "NewEnumerator7")))

(fn `GetReputation`
  (params (`Faction Name` :type Name) (`Target Faction` :type Name))
  (returns (Reputation :type "Float (double-precision)"))
  (bind _faction (`self.GetFaction` `Faction Name`)
    (:`Found`
      (bind (_faction_2 _index) (`self.GetFaction` `Target Faction`)
        (:`Found`
          (return (`|GetArrayItem` (`.Reputations_16_A7D8009747F1AD4E22A5A4B295B4667E` (break `/Game/UniversalMonster/Blueprints/Structs/S_Faction` _faction)) _index)))
        (:`NotFound`
          _)))
    (:`NotFound`
      _))
  (return 0.0))

(fn `InitializeFactions`
  (params (FactionsDT :type "DataTable Object Reference"))
  (if (not (`KismetArrayLibrary.Array_IsValidIndex` (`self.Factions`)))
    (bind _outrownames (`DataTableFunctionLibrary.GetDataTableRowNames` FactionsDT))
    (for _array_element _outrownames
      (bind _returnvalue (`|GetDataTableRow` FactionsDT _array_element)
        (:`then`
          (`KismetArrayLibrary.Array_AddUnique` (`self.Factions`) _returnvalue))))
    (`GameplayStatics.SaveGameToSlot` self (`self.SlotName`))))

(fn `InitializeStats`
  (params (StatsDT :type "DataTable Object Reference"))
  (if (not (`KismetArrayLibrary.Array_IsValidIndex` (`self.Stats`)))
    (bind _outrownames (`DataTableFunctionLibrary.GetDataTableRowNames` StatsDT))
    (for _array_element _outrownames
      (bind _returnvalue (`|GetDataTableRow` StatsDT _array_element)
        (:`then`
          (`KismetArrayLibrary.Array_AddUnique` (`self.Stats`) _returnvalue))))
    (`GameplayStatics.SaveGameToSlot` self (`self.SlotName`))))

(fn `RemoveFaction`
  (params (`Faction Name` :type Name))
  (locals (FactionIndex :type Integer :default 0))
  (bind (_faction _index) (`self.GetFaction` `Faction Name`)
    (:`Found`
      (set `local.FactionIndex` _index)
      (`KismetArrayLibrary.Array_Remove` (`self.Factions`) (`local.FactionIndex`))
      (for (_ _array_index) (`self.Factions`)
        (`KismetArrayLibrary.Array_Remove` (`.Reputations_16_A7D8009747F1AD4E22A5A4B295B4667E` (break `/Game/UniversalMonster/Blueprints/Structs/S_Faction` (`|GetArrayItem` (`self.Factions`) _array_index))) (`local.FactionIndex`)))
      (`GameplayStatics.SaveGameToSlot` self (`self.SlotName`)))))